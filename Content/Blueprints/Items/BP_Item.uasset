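; BP_Item is a world item that rides conveyor belts and can be picked up into the player's inventory, taking its mesh from item data.
; A movement timeline positions it along the belt spline, and a second timeline signals spawning the next item.
; It halts behind a stopped item within the spacing interval, even across belts, broadcasting stop/start events.
; At belt end it transfers to the next belt, feeds a building or stops.
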(event Custom|CE_StopMovement
  (if (CallFunction|ConditiontoStop)
    (Utilities|FlowControl|Sequence
      (:then_0
        (Audio|Components|Audio|Stop (Variables|Default|GetTL_Movement))
        (bind _tl_spawnnext (Variables|Default|GetTL_SpawnNext)
          (:then
            (Audio|Components|Audio|Stop _tl_spawnnext))
          (:else)))
      (:then_1
        (Default|CallTLStopped)))))

(event Custom|CE_ForceStop
  (if (Audio|Components|Audio|IsPlaying (Variables|Default|GetTL_Movement))
    (Utilities|FlowControl|Sequence
      (:then_0
        (Audio|Components|Audio|Stop (Variables|Default|GetTL_Movement))
        (bind _tl_spawnnext (Variables|Default|GetTL_SpawnNext)
          (:then
            (Audio|Components|Audio|Stop _tl_spawnnext))
          (:else)))
      (:then_1
        (Default|CallTLStopped)))))

(event Custom|CE_RestartMovement
  (if (not (Audio|Components|Audio|IsPlaying (Variables|Default|GetTL_Movement)))
    (Utilities|FlowControl|Sequence
      (:then_0
        (Audio|Components|Audio|Play (Variables|Default|GetTL_Movement))
        (bind _tl_spawnnext (Variables|Default|GetTL_SpawnNext)
          (:then
            (Audio|Components|Audio|Play _tl_spawnnext))
          (:else)))
      (:then_1
        (Default|CallTLStarted)))))

(event Custom|CE_EndOf%20Belt
  (Variables|Default|SetHasReachedEnd true)
  (bind (_success _out_build _attachpoint) (Default|GetNextBuild (Variables|Default|GetBeltReference)))
  (Utilities|Casting|CastToBP_Builds_Belt _out_build
    (:then
      (Default|ItemMovedtoNextBelt (Variables|Default|GetBeltReference) self))
    (:CastFailed
      (bind _asbp_buildings (Utilities|Casting|CastToBP_Buildings _out_build)
        (:then
          (bind _success_2 (Default|InputfromAttachPoint _asbp_buildings _attachpoint self))
          (if (not _success_2)
            (CallFunction|CEForceStop)))
        (:CastFailed
          (CallFunction|CEForceStop))))))

(event EventBeginPlay
  (Variables|Default|GetBeltReference
    (:then
      (Utilities|FlowControl|Sequence
        (:then_0
          (Default|ItemsAddedtoBelt (Variables|Default|GetBeltReference) self true))
        (:then_1
          (CallFunction|SetupTimeline)
          (Components|Timeline|SetPlayRate (Variables|Default|GetTL_SpawnNext) (/ (Variables|Default|GetItemInterval) (Variables|/Game/Blueprints/Buildings/Buildables/BP_Builds_Belt.BP_Builds_Belt_C|GetBeltSpeed (Variables|Default|GetBeltReference))))
          (Utilities|FlowControl|DelayUntilNextTick)
          (Timeline|TL_SpawnNext PlayFromStart
            (:Finished
              (Default|CallSpawnNext)
              (Components|DestroyComponent (Variables|Default|GetTL_SpawnNext)))))))
    (:else)))

(fn ConstructionScript
  (bind _staticmesh (Variables|Default|GetStaticMesh))
  (bind _itemdata (Variables|Default|GetItemData))
  (bind _overridematerial (Variables|/Game/Blueprints/Items/DA_Items.DA_Items_C|GetOverrideMaterial (.itemdata _itemdata)))
  (Utilities|IsValid (.itemdata _itemdata)
    (:Is%20Valid
      (Components|StaticMesh|SetStaticMesh _staticmesh (Variables|/Game/Blueprints/Items/DA_Items.DA_Items_C|GetStaticMesh (.itemdata _itemdata)))
      (Utilities|IsValid _overridematerial
        (:Is%20Valid
          (Rendering|Material|SetMaterial _staticmesh 0 _overridematerial))))))

(fn ConditiontoStop
  (if (== (Variables|BP_Item_C|GetBeltReference (Variables|Default|GetItemInFront)) (Variables|Default|GetBeltReference))
    (LocalVariables|SetLocalDistance (- (CallFunction|GetDistanceAlongSpline (Variables|Default|GetItemInFront)) (CallFunction|GetDistanceAlongSpline)))
    (else
      (bind _out_build (Default|GetNextBuild (Variables|Default|GetBeltReference)))
      (if (== _out_build (Variables|BP_Item_C|GetBeltReference (Variables|Default|GetItemInFront)))
        (LocalVariables|SetLocalDistance (+ (CallFunction|GetDistanceAlongSpline (Variables|Default|GetItemInFront)) (- (Spline|GetSplineLength (Variables|/Game/Blueprints/Buildings/Buildables/BP_Builds_Belt.BP_Builds_Belt_C|GetSpline (Variables|Default|GetBeltReference))) (CallFunction|GetDistanceAlongSpline))))
        (else
          (return false)))))
  (if (> (LocalVariables|GetLocalDistance) 0.0)
    (return (and (< (LocalVariables|GetLocalDistance) (Variables|Default|GetItemInterval)) (CallFunction|IsStopped (Variables|Default|GetItemInFront))))
    (else
      (return false))))

(fn BindEvents
  (params (Binding :type BP%20Item%20Object%20Reference))
  (Utilities|IsValid Binding
    (:Is%20Valid
      (EventDispatchers|BindEventtoTLStopped Binding (EventDispatchers|CreateEvent :!event Custom|CE_StopMovement))
      (EventDispatchers|BindEventtoTLStarted Binding (EventDispatchers|CreateEvent :!event Custom|CE_RestartMovement)))))

(fn IsStopped
  (return (not (Audio|Components|Audio|IsPlaying (Variables|Default|GetTL_Movement)))))

(fn IsLastItem
  (return (== (Variables|/Game/Blueprints/Buildings/Buildables/BP_Builds_Belt.BP_Builds_Belt_C|GetLastItemInQueue (Variables|Default|GetBeltReference)) self)))

(fn SetupTimeline
  (params (NewBelt :type BP%20Builds%20Belt%20Object%20Reference))
  (Variables|Default|SetHasReachedEnd false)
  (Utilities|FlowControl|Sequence
    (:then_0
      (bind _newbelt (LocalVariables|GetNewBelt)
        (:then
          (Variables|Default|SetBeltReference _newbelt))
        (:else)))
    (:then_1
      (Components|Timeline|SetPlaybackPosition (Variables|Default|GetTL_Movement) 0.0 false false)
      (Components|Timeline|SetPlayRate (Variables|Default|GetTL_Movement) (|CalculatePlayRate))
      (CallFunction|CERestartMovement))))

(fn GetDistanceAlongSpline
  (return (Default|GetLengthbyAlpha (Variables|Default|GetBeltReference) (Variables|Default|GetAlpha))))

(fn ModifyQuantity
  (params (NewQuantity :type Integer))
  (Utilities|Struct|SetmembersinFInventorySlotStruct (Variables|Default|GetItemData) NewQuantity))

(fn InteractHover
  (bind _itemdata (Variables|Default|GetItemData))
  (bind _name (Variables|/Game/Blueprints/Items/DA_Items.DA_Items_C|GetName (.itemdata _itemdata)))
  (Utilities|IsValid (.itemdata (Variables|Default|GetItemData))
    (:Is%20Valid
      (return (Utilities|String|SelectText (Utilities|Text|FormatText "Pickup {item}" _name) (Utilities|Text|FormatText "Pickup {quantity} {item}" (.quantity _itemdata) _name) (<= (.quantity _itemdata) 1))))
    (:Is%20Not%20Valid
      (return "Pickup ? Item"))))

(fn Interactwith
  (params (PlayerCharacter :type BP%20Factory%20FPS%20Character%20Object%20Reference))
  (bind _itemdata (Variables|Default|GetItemData))
  (bind _success (Default|AddtoInventory (Variables|/Game/Blueprints/Player/BP_FactoryFPSCharacter.BP_FactoryFPSCharacter_C|GetBPC_InventorySystem PlayerCharacter) (.itemdata _itemdata) (.quantity _itemdata)))
  (if _success
    (Utilities|FlowControl|Sequence
      (:then_0
        (bind _beltreference (Variables|Default|GetBeltReference)
          (:then
            (Default|ItemPickedUp _beltreference self false))
          (:else
            (Actor|DestroyActor))))
      (:then_1
        (return true)))
    (else
      (return false))))