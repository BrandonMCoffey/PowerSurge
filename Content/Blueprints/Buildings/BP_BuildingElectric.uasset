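; BP_BuildingElectric is a crafting building that needs and consumes electrical power to run its recipe.
; CanCraft requires enough energy from the BSCElectricNode when EnergyConsumption is positive, and crafting start/stop switches the node's consumed power on or off.
; An attached crafting slot widget shows progress and output item quantity via event bindings, appearing only while a valid recipe is set.
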(event Custom|UpdateWidgetPercent
  (params (Percent :type Float%20%28double-precision%29))
  (Default|UpdateProgressCustom (Variables|Default|GetCraftingWidget) Percent))

(event EventBeginPlay
  (|CallParentFunction)
  (bind _aswb_crafting_item_slot (Utilities|Casting|CastToWB_CraftingItemSlot (UserInterface|GetWidget (Variables|Default|GetWidget))))
  (Variables|Default|SetCraftingWidget _aswb_crafting_item_slot)
  (EventDispatchers|BindEventtoUpdateCraftingProgress (delegate Custom|UpdateWidgetPercent))
  (EventDispatchers|BindEventtoBuildingItemsUpdated (EventDispatchers|CreateEvent :!event UpdateWidgetItems)))

(fn ConstructionScript
  (|CallParentFunction))

(fn CanCraft
  (if (> (Variables|Default|GetEnergyConsumption) 0.0)
    (if (Default|HasEnoughEnergy (Variables|Default|GetBSC_ElectricNode))
      _
      (else
        (return false))))
  (return (|CallParentFunction)))

(fn OnCraftingStartStop
  (params (Crafting :type Boolean))
  (Variables|/Game/Blueprints/Buildings/BSC_ElectricNode.BSC_ElectricNode_C|SetPowerConsumed (Variables|Default|GetBSC_ElectricNode) (Math|Float|SelectFloat (Variables|Default|GetEnergyConsumption) 0.0 Crafting))
  (|CallParentFunction Crafting))

(fn PlaceBuild
  (Development|SetHiddeninGame (Variables|Default|GetWidget) (not (Utilities|IsValid (Variables|Default|GetRecipe))) false)
  (bind _success (|CallParentFunction))
  (return _success))

(fn ChangeRecipe
  (params (NewRecipe :type DA%20Recipe%20Object%20Reference))
  (|CallParentFunction NewRecipe)
  (Utilities|IsValid (Variables|Default|GetRecipe)
    (:Is%20Valid
      (Development|SetHiddeninGame (Variables|Default|GetWidget) false false)
      (CallFunction|UpdateWidgetItems))
    (:Is%20Not%20Valid
      (Development|SetHiddeninGame (Variables|Default|GetWidget) true false))))

(fn UpdateWidgetItems
  (bind _recipe (Variables|Default|GetRecipe))
  (bind _output (Default|FirstOutput _recipe))
  (bind _values (Utilities|Map|Values (Variables|Default|GetOutputs)))
  (Default|UpdateBasicAppearance (Variables|Default|GetCraftingWidget) (Utilities|Struct|MakeFInventorySlotStruct (.itemdata _output) (.quantity (Utilities|Array|Get(acopy) _values))) (Variables|/Game/Blueprints/Items/DA_Items.DA_Items_C|GetMaxStack (.itemdata _output))))