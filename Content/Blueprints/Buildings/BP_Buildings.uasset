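; Base factory building that turns recipe inputs into outputs and exchanges items with conveyor belts.
; Child attach points key the Input and Output slot maps; slot changes re-check crafting, which runs on a timeline rate-scaled by recipe duration.
; Finished crafts spawn items onto connected belts; rejected incoming items are remembered and restarted when accepted.
; Changing recipe returns mismatched items to the player's inventory, and interacting opens the building's edit menu.
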(event Custom|CE_StartCrafting
  (Crafting|OnCraftingStartStop true)
  (bind _alpha (Timeline|TL_Crafting PlayFromStart)
    (:Update
      (Default|CallUpdateCraftingProgress _alpha))
    (:Finished
      (Utilities|FlowControl|Sequence
        (:then_0
          (Crafting|ConsumeInputItems)
          (Crafting|SendCraftedtoOutput)
          (Output|StartOutputting)
          (Components|Timeline|SetPlaybackPosition (Variables|Default|GetTL_Crafting) 0.0 false true)
          (Default|CallFinishedCrafting))
        (:then_1
          (if (Crafting|CanCraft)
            (CallFunction|CEStartCrafting)))))))

(event Custom|CE_ResumeCrafting
  (Crafting|OnCraftingStartStop true)
  (bind _alpha (Timeline|TL_Crafting Play)
    (:Update
      (Default|CallUpdateCraftingProgress _alpha))
    (:Finished
      (Utilities|FlowControl|Sequence
        (:then_0
          (Crafting|ConsumeInputItems)
          (Crafting|SendCraftedtoOutput)
          (Output|StartOutputting)
          (Components|Timeline|SetPlaybackPosition (Variables|Default|GetTL_Crafting) 0.0 false true)
          (Default|CallFinishedCrafting))
        (:then_1
          (if (Crafting|CanCraft)
            (CallFunction|CEStartCrafting)))))))

(event Custom|CE_StopCrafting
  (Crafting|OnCraftingStartStop false)
  (Utilities|FlowControl|Sequence
    (:then_0
      (bind _alpha (Timeline|TL_Crafting Stop)
        (:Update
          (Default|CallUpdateCraftingProgress _alpha))
        (:Finished
          (Utilities|FlowControl|Sequence
            (:then_0
              (Crafting|ConsumeInputItems)
              (Crafting|SendCraftedtoOutput)
              (Output|StartOutputting)
              (Components|Timeline|SetPlaybackPosition (Variables|Default|GetTL_Crafting) 0.0 false true)
              (Default|CallFinishedCrafting))
            (:then_1
              (if (Crafting|CanCraft)
                (CallFunction|CEStartCrafting)))))))
    (:then_1
      (Timeline|TL_Crafting SetNewTime))))

(event EventBeginPlay
  (|CallParentFunction)
  (for _array_element (Actor|GetAllChildActors true)
    (bind _asbp_attach_point (Utilities|Casting|CastToBP_AttachPoint _array_element))
    (Variables|/Game/Blueprints/Buildings/BP_AttachPoint.BP_AttachPoint_C|SetParentBuild _asbp_attach_point self)
    (switch Utilities|FlowControl|Switch|SwitchonEDirectionEnum (Variables|/Game/Blueprints/Buildings/BP_AttachPoint.BP_AttachPoint_C|GetDirection _asbp_attach_point)
      (:NewEnumerator1
        (Utilities|Map|Add :TargetMap (Variables|Input|GetInputs) :Key _asbp_attach_point))
      (:NewEnumerator2
        (Utilities|Map|Add :TargetMap (Variables|Output|GetOutputs) :Key _asbp_attach_point)))))

(fn ConstructionScript
  (|CallParentFunction))

(fn BeltAttachedOutput
  (params (AttachPoint :type BP%20Attach%20Point%20Object%20Reference))
  (Utilities|Casting|CastToBP_Builds_Belt (Variables|/Game/Blueprints/Buildings/BP_AttachPoint.BP_AttachPoint_C|GetConnectedBuild AttachPoint)
    (:then
      (Output|StartOutputting)
      (return))
    (:CastFailed
      (return))))

(fn StartOutputting
  (bind _keys (Utilities|Map|Keys (Variables|Output|GetOutputs)))
  (for _array_element _keys
    (if (> (.Quantity (Utilities|Struct|BreakFInventorySlotStruct (.Value (Utilities|Map|Find (Variables|Output|GetOutputs) _array_element)))) 0)
      (bind _success (Output|OutputfromAttachPoint _array_element (.ItemData (Utilities|Struct|BreakFInventorySlotStruct (.Value (Utilities|Map|Find (Variables|Output|GetOutputs) _array_element))))))
      (if _success
        (Output|ModifyOutputMap _array_element (Assist|ModifyItemQuantity (.Value (Utilities|Map|Find (Variables|Output|GetOutputs) _array_element)) -1))))))

(fn CanOutputItem
  (return true))

(fn OutputfromAttachPoint
  (params (AttachPoint :type BP%20Attach%20Point%20Object%20Reference) (ItemData :type DA%20Items%20Object%20Reference))
  (if (Output|CanOutputItem)
    (bind _asbp_builds_belt (Utilities|Casting|CastToBP_Builds_Belt (Variables|/Game/Blueprints/Buildings/BP_AttachPoint.BP_AttachPoint_C|GetConnectedBuild AttachPoint))
      (:then
        (if (Default|CanSpawnNextItem _asbp_builds_belt)
          (bind _returnvalue (Game|SpawnActorfromClass "/Game/Blueprints/Items/BP_Item.BP_Item_C" (Default|GetTransformbyAlpha _asbp_builds_belt 0.0) "Undefined" "MultiplyWithRoot" 0 (Utilities|Struct|MakeFInventorySlotStruct ItemData 1) _asbp_builds_belt (Variables|Output|GetItemSpawnInterval) 0))
          (EventDispatchers|BindEventtoSpawnNext _returnvalue (EventDispatchers|CreateEvent :!event StartOutputting))
          (Default|CallBuildingItemsUpdated)
          (return true)
          (else
            (return false) ; Wrong Spacing Between Items
          )))
      (:CastFailed
        (return false)))
    (else
      (return false))))

(fn ConveyorAttachedInput
  (params (AttachPoint :type BP%20Attach%20Point%20Object%20Reference)))

(fn CanInputItem
  (params (InputItem :type DA%20Items%20Object%20Reference))
  (Variables|Crafting|GetRecipe
    (:then
      (bind _values (Utilities|Map|Values (Variables|Input|GetInputs)))
      (for _array_element _values
        (Utilities|IsValid (Utilities|Struct|BreakFInventorySlotStruct _array_element)
          (:Is%20Valid
            (if (or (== (.Quantity (Utilities|Struct|BreakFInventorySlotStruct _array_element)) 0) (== (.ItemData (Utilities|Struct|BreakFInventorySlotStruct _array_element)) InputItem))
              (if (Crafting|IsSlotIncomplete _array_element)
                (return true)
                (else
                  (return false)))))
          (:Is%20Not%20Valid
            (for _array_element_2 (Variables|/Game/Blueprints/Items/DA_Recipe.DA_Recipe_C|GetInputs (Variables|Crafting|GetRecipe))
              (if (== (Utilities|Struct|BreakFInventorySlotStruct _array_element_2) InputItem)
                (return true)))
            (return false)))))
    (:else
      (return false))))

(fn InputfromAttachPoint
  (params (AttachPoint :type BP%20Attach%20Point%20Object%20Reference) (InputItem :type BP%20Item%20Object%20Reference))
  (bind _itemdata (Variables|/Game/Blueprints/Items/BP_Item.BP_Item_C|GetItemData InputItem))
  (if (Input|CanInputItem (.itemdata (Variables|/Game/Blueprints/Items/BP_Item.BP_Item_C|GetItemData InputItem)))
    (Utilities|IsValid (Utilities|Struct|BreakFInventorySlotStruct (.Value (Utilities|Map|Find (Variables|Input|GetInputs) AttachPoint)))
      (:Is%20Valid
        (LocalVariables|SetLocalNewStructure (Assist|ModifyItemQuantity (.Value (Utilities|Map|Find (Variables|Input|GetInputs) AttachPoint)) 1)))
      (:Is%20Not%20Valid
        (LocalVariables|SetLocalNewStructure (Utilities|Struct|MakeFInventorySlotStruct (.itemdata _itemdata) (.quantity _itemdata)))))
    (Input|ModifyInputMap AttachPoint (LocalVariables|GetLocalNewStructure))
    (Actor|DestroyActor InputItem)
    (Default|CallBuildingItemsUpdated)
    (if (Output|CanOutputItem)
      (Output|StartOutputting))
    (return true)
    (else
      (Utilities|Map|Add (Variables|Input|GetAttemptedInputs) AttachPoint InputItem)
      (return false))))

(fn ModifyItemQuantity
  (params (ItemSlot :type F%20Inventory%20Slot%20Struct%20Structure) (Modifier :type Integer))
  (bind (_itemdata _quantity) (Utilities|Struct|BreakFInventorySlotStruct ItemSlot))
  (return (Utilities|Struct|MakeFInventorySlotStruct _itemdata (+ _quantity Modifier))))

(fn IsSlotIncomplete
  (params (Slot :type F%20Inventory%20Slot%20Struct%20Structure))
  (bind (_itemdata _quantity) (Utilities|Struct|BreakFInventorySlotStruct Slot))
  (return (< _quantity (Variables|/Game/Blueprints/Items/DA_Items.DA_Items_C|GetMaxStack _itemdata))))

(fn ModifyInputMap
  (params (Key :type BP%20Attach%20Point%20Object%20Reference) (Value :type F%20Inventory%20Slot%20Struct%20Structure%20%28by%20ref%29))
  (Utilities|FlowControl|Sequence
    (:then_0
      (Utilities|IsValid Key
        (:Is%20Valid
          (Utilities|Map|Add (Variables|Input|GetInputs) Key Value))
        (:Is%20Not%20Valid
          (bind _keys (Utilities|Map|Keys (Variables|Input|GetInputs)))
          (bind _array_element (Utilities|Array|ForEachLoopwithBreak _keys :!label _label)
            (:LoopBody
              (if (== (.itemdata Value) (.itemdata (.Value (Utilities|Map|Find (Variables|Input|GetInputs) _array_element))))
                (Utilities|Map|Add (Variables|Input|GetInputs) _array_element Value)
                (goto _label Break)))))))
    (:then_1
      (Crafting|AttemptCrafting))))

(fn CanCraft
  (Variables|Crafting|GetRecipe
    (:then
      (Utilities|FlowControl|Sequence
        (:then_0
          (bind _values (Utilities|Map|Values (Variables|Output|GetOutputs)))
          (for _array_element _values
            (if (not (Crafting|IsSlotIncomplete _array_element))
              (return false))))
        (:then_1
          (if (not (Utilities|Array|IsNotEmpty (Variables|/Game/Blueprints/Items/DA_Recipe.DA_Recipe_C|GetInputs (Variables|Crafting|GetRecipe)))) ; No Inputs, no need to check for available resources
            (return true)))
        (:then_2
          (bind _values_2 (Utilities|Map|Values (Variables|Input|GetInputs)))
          (LocalVariables|SetLocalAvailableResources _values_2)
          (for _array_element_2 (Variables|/Game/Blueprints/Items/DA_Recipe.DA_Recipe_C|GetInputs (Variables|Crafting|GetRecipe))
            (LocalVariables|SetLocalItemRequired (.ItemData (Utilities|Struct|BreakFInventorySlotStruct _array_element_2)))
            (LocalVariables|SetLocalQuantityRequired (.Quantity (Utilities|Struct|BreakFInventorySlotStruct _array_element_2)))
            (LocalVariables|SetLocalFoundItem false)
            (bind _array_element_3 (Utilities|Array|ForEachLoopwithBreak (LocalVariables|GetLocalAvailableResources) :!label _label)
              (:LoopBody
                (if (and (<= (LocalVariables|GetLocalQuantityRequired) (.Quantity (Utilities|Struct|BreakFInventorySlotStruct _array_element_3))) (== (.ItemData (Utilities|Struct|BreakFInventorySlotStruct _array_element_3)) (LocalVariables|GetLocalItemRequired)))
                  (LocalVariables|SetLocalFoundItem true)
                  (goto _label Break)))
              (:Completed
                (if (not (LocalVariables|GetLocalFoundItem))
                  (return false))))))
        (:then_3
          (bind _values_3 (Utilities|Map|Values (Variables|Output|GetOutputs)))
          (LocalVariables|SetLocalAvailableResources _values_3)
          (for _array_element_4 (Variables|/Game/Blueprints/Items/DA_Recipe.DA_Recipe_C|GetOutputs (Variables|Crafting|GetRecipe))
            (LocalVariables|SetLocalItemRequired (.ItemData (Utilities|Struct|BreakFInventorySlotStruct _array_element_4)))
            (LocalVariables|SetLocalQuantityRequired (.Quantity (Utilities|Struct|BreakFInventorySlotStruct _array_element_4)))
            (for _array_element_5 (LocalVariables|GetLocalAvailableResources)
              (if (and (> (+ (LocalVariables|GetLocalQuantityRequired) (.Quantity (Utilities|Struct|BreakFInventorySlotStruct _array_element_5))) (Variables|/Game/Blueprints/Items/DA_Items.DA_Items_C|GetMaxStack (LocalVariables|GetLocalItemRequired))) (== (.ItemData (Utilities|Struct|BreakFInventorySlotStruct _array_element_5)) (LocalVariables|GetLocalItemRequired)))
                (return false)))))
        (:then_4
          (return true))))
    (:else
      (return false))))

(fn SendCraftedtoOutput
  (bind _keys (Utilities|Map|Keys (Variables|Output|GetOutputs)))
  (for _array_element _keys
    (for _array_element_2 (Variables|/Game/Blueprints/Items/DA_Recipe.DA_Recipe_C|GetOutputs (Variables|Crafting|GetRecipe))
      (if (== (.ItemData (Utilities|Struct|BreakFInventorySlotStruct _array_element_2)) (Utilities|Struct|BreakFInventorySlotStruct (.Value (Utilities|Map|Find (Variables|Output|GetOutputs) _array_element))))
        (LocalVariables|SetLocalQuantityToAdd (.Quantity (Utilities|Struct|BreakFInventorySlotStruct _array_element_2)))))
    (Utilities|Map|Add (Variables|Output|GetOutputs) _array_element (Assist|ModifyItemQuantity (.Value (Utilities|Map|Find (Variables|Output|GetOutputs) _array_element)) (LocalVariables|GetLocalQuantityToAdd)))))

(fn ConsumeInputItems
  (bind _keys (Utilities|Map|Keys (Variables|Input|GetInputs)))
  (for _array_element _keys
    (LocalVariables|SetLocalAttachPoint _array_element)
    (LocalVariables|SetLocalInputItem (.Value (Utilities|Map|Find (Variables|Input|GetInputs) _array_element)))
    (bind _array_element_2 (Utilities|Array|ForEachLoopwithBreak (Variables|/Game/Blueprints/Items/DA_Recipe.DA_Recipe_C|GetInputs (Variables|Crafting|GetRecipe)) :!label _label)
      (:LoopBody
        (if (== (.ItemData (Utilities|Struct|BreakFInventorySlotStruct _array_element_2)) (.itemdata (LocalVariables|GetLocalInputItem)))
          (Utilities|Map|Add (Variables|Input|GetInputs) (LocalVariables|GetLocalAttachPoint) (Assist|ModifyItemQuantity (LocalVariables|GetLocalInputItem) (* (.Quantity (Utilities|Struct|BreakFInventorySlotStruct _array_element_2)) -1)))
          (goto _label Break)))))
  (bind _keys_2 (Utilities|Map|Keys (Variables|Input|GetAttemptedInputs)))
  (for _array_element_3 _keys_2
    (Utilities|IsValid (.Value (Utilities|Map|Find (Variables|Input|GetAttemptedInputs) _array_element_3))
      (:Is%20Valid
        (if (Input|CanInputItem (.itemdata (Variables|/Game/Blueprints/Items/BP_Item.BP_Item_C|GetItemData (.Value (Utilities|Map|Find (Variables|Input|GetAttemptedInputs) _array_element_3)))))
          (Default|CERestartMovement (.Value (Utilities|Map|Find (Variables|Input|GetAttemptedInputs) _array_element_3))))))))

(fn ChangeRecipe
  (params (NewRecipe :type DA%20Recipe%20Object%20Reference))
  (if (!= NewRecipe (Variables|Crafting|GetRecipe))
    (Variables|Crafting|SetRecipe NewRecipe)
    (Utilities|FlowControl|Sequence
      (:then_0
        (bind _asbp_factory_fpscharacter (Utilities|Casting|CastToBP_FactoryFPSCharacter (Game|Player|GetPlayerPawn 0)))
        (LocalVariables|SetPlayerInventory (Variables|/Game/Blueprints/Player/BP_FactoryFPSCharacter.BP_FactoryFPSCharacter_C|GetBPC_InventorySystem _asbp_factory_fpscharacter))
        (Utilities|FlowControl|Sequence
          (:then_0
            (bind _keys (Utilities|Map|Keys (Variables|Input|GetInputs)))
            (for (_array_element _array_index) _keys
              (if (and (!= (.itemdata (.Value (Utilities|Map|Find (Variables|Input|GetInputs) _array_element))) (.itemdata (Utilities|Array|Get(acopy) (Variables|/Game/Blueprints/Items/DA_Recipe.DA_Recipe_C|GetInputs (Variables|Crafting|GetRecipe)) _array_index))) (> (.quantity (.Value (Utilities|Map|Find (Variables|Input|GetInputs) _array_element))) 0))
                (Default|AddtoInventory (LocalVariables|GetPlayerInventory) (.itemdata (.Value (Utilities|Map|Find (Variables|Input|GetInputs) _array_element))) (.quantity (.Value (Utilities|Map|Find (Variables|Input|GetInputs) _array_element)))))
              (Utilities|Map|Add (Variables|Input|GetInputs) _array_element (Utilities|Struct|MakeFInventorySlotStruct (.itemdata (Utilities|Array|Get(acopy) (Variables|/Game/Blueprints/Items/DA_Recipe.DA_Recipe_C|GetInputs (Variables|Crafting|GetRecipe)) _array_index)) 0))))
          (:then_1
            (bind _keys_2 (Utilities|Map|Keys (Variables|Output|GetOutputs)))
            (for (_array_element_2 _array_index_2) _keys_2
              (if (and (!= (.itemdata (.Value (Utilities|Map|Find (Variables|Output|GetOutputs) _array_element_2))) (.itemdata (Utilities|Array|Get(acopy) (Variables|/Game/Blueprints/Items/DA_Recipe.DA_Recipe_C|GetOutputs (Variables|Crafting|GetRecipe)) _array_index_2))) (> (.quantity (.Value (Utilities|Map|Find (Variables|Output|GetOutputs) _array_element_2))) 0))
                (Default|AddtoInventory (LocalVariables|GetPlayerInventory) (.itemdata (.Value (Utilities|Map|Find (Variables|Output|GetOutputs) _array_element_2))) (.quantity (.Value (Utilities|Map|Find (Variables|Output|GetOutputs) _array_element_2)))))
              (Utilities|Map|Add (Variables|Output|GetOutputs) _array_element_2 (Utilities|Struct|MakeFInventorySlotStruct (.itemdata (Utilities|Array|Get(acopy) (Variables|/Game/Blueprints/Items/DA_Recipe.DA_Recipe_C|GetOutputs (Variables|Crafting|GetRecipe)) _array_index_2)) 0))))))
      (:then_1
        (Crafting|AttemptCrafting)
        (bind _recipe (Variables|Crafting|GetRecipe)
          (:then
            (Components|Timeline|SetPlayRate (Variables|Default|GetTL_Crafting) (/ 1.0 (Variables|/Game/Blueprints/Items/DA_Recipe.DA_Recipe_C|GetDuration _recipe))))
          (:else)))
      (:then_2
        (bind _keys_3 (Utilities|Map|Keys (Variables|Input|GetAttemptedInputs)))
        (for _array_element_3 _keys_3
          (Utilities|IsValid (.Value (Utilities|Map|Find (Variables|Input|GetAttemptedInputs) _array_element_3))
            (:Is%20Valid
              (if (Input|CanInputItem (.itemdata (Variables|/Game/Blueprints/Items/BP_Item.BP_Item_C|GetItemData (.Value (Utilities|Map|Find (Variables|Input|GetAttemptedInputs) _array_element_3)))))
                (Default|CERestartMovement (.Value (Utilities|Map|Find (Variables|Input|GetAttemptedInputs) _array_element_3)))))))))))

(fn ModifyOutputMap
  (params (Key :type BP%20Attach%20Point%20Object%20Reference) (Value :type F%20Inventory%20Slot%20Struct%20Structure%20%28by%20ref%29))
  (Utilities|FlowControl|Sequence
    (:then_0
      (Utilities|IsValid Key
        (:Is%20Valid
          (Utilities|Map|Add (Variables|Output|GetOutputs) Key Value))
        (:Is%20Not%20Valid
          (bind _keys (Utilities|Map|Keys (Variables|Output|GetOutputs)))
          (bind _array_element (Utilities|Array|ForEachLoopwithBreak _keys :!label _label)
            (:LoopBody
              (if (== (.itemdata Value) (.itemdata (.Value (Utilities|Map|Find (Variables|Output|GetOutputs) _array_element))))
                (Utilities|Map|Add (Variables|Output|GetOutputs) _array_element Value)
                (goto _label Break)))))))
    (:then_1
      (Crafting|AttemptCrafting))))

(fn AttemptCrafting
  (if (Crafting|CanCraft)
    (if (not (Audio|Components|Audio|IsPlaying (Variables|Default|GetTL_Crafting)))
      (CallFunction|CEResumeCrafting))
    (elif (Audio|Components|Audio|IsPlaying (Variables|Default|GetTL_Crafting))
      (CallFunction|CEStopCrafting))))

(fn CanOutputfromAttachPoint
  (params (AttachPoint :type BP%20Attach%20Point%20Object%20Reference))
  (bind _connectedbuild (Variables|/Game/Blueprints/Buildings/BP_AttachPoint.BP_AttachPoint_C|GetConnectedBuild AttachPoint)
    (:then
      (bind _asbp_builds_belt (Utilities|Casting|CastToBP_Builds_Belt _connectedbuild)
        (:then
          (return (Default|CanSpawnNextItem _asbp_builds_belt)))
        (:CastFailed
          _)))
    (:else
      _))
  (return false))

(fn PlaceBuild
  (bind _success (|CallParentFunction))
  (Utilities|FlowControl|Sequence
    (:then_0
      (bind _keys (Utilities|Map|Keys (Variables|Input|GetInputs)))
      (for _array_element _keys
        (Default|UpdateArrowColor _array_element)))
    (:then_1
      (bind _keys_2 (Utilities|Map|Keys (Variables|Output|GetOutputs)))
      (for _array_element_2 _keys_2
        (Default|UpdateArrowColor _array_element_2)))
    (:then_2
      (return _success))))

(fn OnCraftingStartStop
  (params (Crafting :type Boolean)))

(fn GetClosestAttachPoint
  (params (WorldLocation :type Vector) (BeltDirection :type EDirectionEnum%20Enum :default "NewEnumerator0"))
  (LocalVariables|SetLocalDistance 0.0)
  (Utilities|FlowControl|Sequence
    (:then_0
      (bind _keys (Utilities|Map|Keys (Variables|Input|GetInputs)))
      (for _array_element _keys
        (if (Default|CanConveyorConnect _array_element BeltDirection)
          (if (or (== (LocalVariables|GetLocalDistance) 0.0) (< (Math|Vector|Distance(Vector) (Transformation|GetWorldLocation (Variables|/Game/Blueprints/Buildings/BP_AttachPoint.BP_AttachPoint_C|GetDefaultSceneRoot _array_element)) WorldLocation) (LocalVariables|GetLocalDistance)))
            (LocalVariables|SetLocalDistance (Math|Vector|Distance(Vector) (Transformation|GetWorldLocation (Variables|/Game/Blueprints/Buildings/BP_AttachPoint.BP_AttachPoint_C|GetDefaultSceneRoot _array_element)) WorldLocation))
            (LocalVariables|SetLocalAttachPoint _array_element)))))
    (:then_1
      (bind _keys_2 (Utilities|Map|Keys (Variables|Output|GetOutputs)))
      (for _array_element_2 _keys_2
        (if (Default|CanConveyorConnect _array_element_2 BeltDirection)
          (if (or (== (LocalVariables|GetLocalDistance) 0.0) (< (Math|Vector|Distance(Vector) (Transformation|GetWorldLocation (Variables|/Game/Blueprints/Buildings/BP_AttachPoint.BP_AttachPoint_C|GetDefaultSceneRoot _array_element_2)) WorldLocation) (LocalVariables|GetLocalDistance)))
            (LocalVariables|SetLocalDistance (Math|Vector|Distance(Vector) (Transformation|GetWorldLocation (Variables|/Game/Blueprints/Buildings/BP_AttachPoint.BP_AttachPoint_C|GetDefaultSceneRoot _array_element_2)) WorldLocation))
            (LocalVariables|SetLocalAttachPoint _array_element_2)))))
    (:then_2
      (LocalVariables|GetLocalAttachPoint
        (:then
          (return true (LocalVariables|GetLocalAttachPoint)))
        (:else
          (return false 0))))))

(fn InteractHover
  (bind _buildingdata (Variables|Default|GetBuildingData))
  (Utilities|IsValid _buildingdata
    (:Is%20Valid
      (return (Utilities|Text|FormatText "Open {Building}" (Variables|/Game/Blueprints/Buildings/DA_Buildable.DA_Buildable_C|GetName _buildingdata))))
    (:Is%20Not%20Valid
      (return "Open Building"))))

(fn Interactwith
  (params (PlayerCharacter :type BP%20Factory%20FPS%20Character%20Object%20Reference))
  (bind (_success _hud) (Default|GetHud PlayerCharacter))
  (if _success
    (Default|OpenMenuEditBuilding _hud self)
    (return true)
    (else
      (return false))))