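; Buildable electric cable that is placed in two steps, linking a start and an end electric node with a spline mesh.
; Each step previews a hologram BP_Builds_ElectricPole, which is hidden when the cursor hits an existing node to snap to, and otherwise gets built.
; StartPlaced switches update, validation and placement between the two ends.
; Validation checks node capacity and duplicate links; placement connects the cable and destruction disconnects it.
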(fn ConstructionScript
  (|CallParentFunction))

(fn UpdateLocation
  (params (HitInformation :type Hit%20Result%20Structure))
  (bind _endpole (Variables|Default|GetEndPole))
  (bind _hitactor (Collision|BreakHitResult HitInformation))
  (bind _hitactor_2 (Collision|BreakHitResult HitInformation))
  (bind _returnvalue (Actor|GetComponentbyClass _hitactor "/Game/Blueprints/Buildings/BSC_ElectricNode.BSC_ElectricNode_C"))
  (bind _returnvalue_2 (Actor|GetComponentbyClass _hitactor_2 "/Game/Blueprints/Buildings/BSC_ElectricNode.BSC_ElectricNode_C"))
  (Variables|Default|SetValidLocation true)
  (Utilities|IsStartPlaced
    (:IsPlaced
      (Utilities|FlowControl|Sequence
        (:then_0
          (bind _asbp_builds_electric_pole (Utilities|Casting|CastToBP_Builds_ElectricPole (.HitActor (Collision|BreakHitResult HitInformation)))
            (:then
              (if (!= (Variables|Default|GetEndPole) _asbp_builds_electric_pole)
                (bind _overlappingpole (Variables|Default|GetOverlappingPole)
                  (:then
                    (if (not (== _overlappingpole _asbp_builds_electric_pole))
                      (Default|HideWidget _overlappingpole)
                      (bind _startconnect (Variables|Default|GetStartConnect :!label _label)
                        (:then
                          (if (not (Utilities|Set|Contains (Variables|/Game/Blueprints/Buildings/BSC_ElectricNode.BSC_ElectricNode_C|GetConnectedNodes _startconnect) (Variables|/Game/Blueprints/Buildings/Buildables/BP_Builds_ElectricPole.BP_Builds_ElectricPole_C|GetBSC_ElectricNode _asbp_builds_electric_pole)))
                            (bind _output_get (Variables|Default|SetOverlappingPole _asbp_builds_electric_pole :!label _label_2))
                            (Default|DisplayWidget _output_get)
                            (Variables|Default|SetEndConnect (Variables|/Game/Blueprints/Buildings/Buildables/BP_Builds_ElectricPole.BP_Builds_ElectricPole_C|GetBSC_ElectricNode _asbp_builds_electric_pole))))
                        (:else
                          (goto _label_2)))))
                  (:else
                    (goto _label)))))
            (:CastFailed
              (bind _overlappingpole_2 (Variables|Default|GetOverlappingPole)
                (:then
                  (Default|HideWidget _overlappingpole_2)
                  (Variables|Default|SetOverlappingPole 0)
                  (Variables|Default|SetEndConnect 0))
                (:else)))))
        (:then_1
          (Utilities|IsValid _returnvalue_2
            (:Is%20Valid
              (if (!= _hitactor_2 (Variables|Default|GetEndPole))
                (Variables|Default|SetEndConnect _returnvalue_2)
                (LocalVariables|SetLocalTargetLocation (Math|Transform|InverseTransformLocation (Transformation|GetActorTransform) (Transformation|GetWorldLocation _returnvalue_2)))
                (Rendering|SetActorHiddenInGame (Variables|Default|GetEndPole) true)
                (else
                  (CallFunction|UpdateLocation _endpole HitInformation :!label _label_3)
                  (LocalVariables|SetLocalTargetLocation (Math|Transform|InverseTransformLocation (Transformation|GetActorTransform) (Transformation|GetWorldLocation (Variables|/Game/Blueprints/Buildings/Buildables/BP_Builds_ElectricPole.BP_Builds_ElectricPole_C|GetBSC_ElectricNode _endpole))))
                  (Rendering|SetActorHiddenInGame (Variables|Default|GetEndPole) false))))
            (:Is%20Not%20Valid
              (goto _label_3))))
        (:then_2
          (SplineMesh|SetStartandEnd (Variables|Default|GetSplineMesh) "0, 0, 0" "0, 0, 0" (LocalVariables|GetLocalTargetLocation) "0, 0, 0" true :!class /Script/Engine.SplineMeshComponent))))
    (:IsNotPlaced
      (Utilities|FlowControl|Sequence
        (:then_0
          (bind _asbp_builds_electric_pole_2 (Utilities|Casting|CastToBP_Builds_ElectricPole (.HitActor (Collision|BreakHitResult HitInformation)))
            (:then
              (if (!= (Variables|Default|GetStartPole) _asbp_builds_electric_pole_2)
                (bind _overlappingpole_3 (Variables|Default|GetOverlappingPole)
                  (:then
                    (if (not (== _overlappingpole_3 _asbp_builds_electric_pole_2))
                      (Default|HideWidget _overlappingpole_3)
                      (bind _output_get_2 (Variables|Default|SetOverlappingPole _asbp_builds_electric_pole_2 :!label _label_4))
                      (Default|DisplayWidget _output_get_2)
                      (Variables|Default|SetStartConnect (Variables|/Game/Blueprints/Buildings/Buildables/BP_Builds_ElectricPole.BP_Builds_ElectricPole_C|GetBSC_ElectricNode _asbp_builds_electric_pole_2))))
                  (:else
                    (goto _label_4)))))
            (:CastFailed
              (bind _overlappingpole_4 (Variables|Default|GetOverlappingPole)
                (:then
                  (Default|HideWidget _overlappingpole_4)
                  (Variables|Default|SetOverlappingPole 0)
                  (Variables|Default|SetStartConnect 0))
                (:else)))))
        (:then_1
          (Utilities|IsValid _returnvalue
            (:Is%20Valid
              (if (!= _hitactor (Variables|Default|GetStartPole))
                (Utilities|Array|Add (Variables|Default|GetActors%20to%20Ignore) _hitactor)
                (Variables|Default|SetStartConnect _returnvalue)
                (Transformation|SetActorLocation (Transformation|GetWorldLocation (Variables|Default|GetStartConnect)) false false)
                (Rendering|SetActorHiddenInGame (Variables|Default|GetStartPole) true)
                (else
                  (CallFunction|UpdateLocation (Variables|Default|GetStartPole) HitInformation :!label _label_5)
                  (Transformation|SetActorLocation (Transformation|GetWorldLocation (Variables|/Game/Blueprints/Buildings/Buildables/BP_Builds_ElectricPole.BP_Builds_ElectricPole_C|GetBSC_ElectricNode (Variables|Default|GetStartPole))) false false)
                  (Rendering|SetActorHiddenInGame (Variables|Default|GetStartPole) false))))
            (:Is%20Not%20Valid
              (goto _label_5))))))))

(fn PlaceBuild
  (bind _startpole (Variables|Default|GetStartPole))
  (Utilities|IsStartPlaced
    (:IsPlaced
      (Utilities|FlowControl|Sequence
        (:then_0
          (if (Variables|/Script/Engine.Actor|GetbHidden (Variables|Default|GetStartPole))
            (Actor|DestroyActor (Variables|Default|GetStartPole)))
          (if (Variables|/Script/Engine.Actor|GetbHidden (Variables|Default|GetEndPole))
            (Actor|DestroyActor (Variables|Default|GetEndPole))
            (else
              (CallFunction|PlaceBuild (Variables|Default|GetEndPole)))))
        (:then_1
          (Utilities|FlowControl|Sequence
            (:then_0
              (bind _startpole_2 (Variables|Default|GetStartPole)
                (:then
                  (Variables|Default|SetStartConnect (Variables|/Game/Blueprints/Buildings/Buildables/BP_Builds_ElectricPole.BP_Builds_ElectricPole_C|GetBSC_ElectricNode _startpole_2)))
                (:else)))
            (:then_1
              (bind _endpole (Variables|Default|GetEndPole)
                (:then
                  (Variables|Default|SetEndConnect (Variables|/Game/Blueprints/Buildings/Buildables/BP_Builds_ElectricPole.BP_Builds_ElectricPole_C|GetBSC_ElectricNode _endpole)))
                (:else)))
            (:then_2
              (Default|ConnectCable (Variables|Default|GetEndConnect) self)
              (|CallParentFunction)
              (return true))))))
    (:IsNotPlaced
      (Variables|Default|SetStartPlaced true)
      (Development|SetHiddeninGame (Variables|Default|GetSplineMesh) false false)
      (Utilities|FlowControl|Sequence
        (:then_0
          (if (not (Variables|/Script/Engine.Actor|GetbHidden (Variables|Default|GetStartPole)))
            (CallFunction|PlaceBuild _startpole)
            (Variables|Default|SetStartConnect (Variables|/Game/Blueprints/Buildings/Buildables/BP_Builds_ElectricPole.BP_Builds_ElectricPole_C|GetBSC_ElectricNode _startpole))))
        (:then_1
          (bind _returnvalue (Game|SpawnActorfromClass "/Game/Blueprints/Buildings/Buildables/BP_Builds_ElectricPole.BP_Builds_ElectricPole_C" (Transformation|GetActorTransform) "Undefined" "MultiplyWithRoot" 0 0 0))
          (bind _output_get (Variables|Default|SetEndPole _returnvalue))
          (Default|SetAllMaterials _output_get "/Game/Assets/Holograms/M_HologramPlace.M_HologramPlace" false)
          (Default|UpdateCollision _output_get "NoCollision")
          (Utilities|Array|Add (Variables|Default|GetActors%20to%20Ignore) _output_get)
          (Variables|Default|SetOverlappingPole 0)
          (return false))))))

(fn CreateBuild
  (bind _returnvalue (Game|SpawnActorfromClass "/Game/Blueprints/Buildings/Buildables/BP_Builds_ElectricPole.BP_Builds_ElectricPole_C" (Transformation|GetActorTransform) "Undefined" "MultiplyWithRoot" 0 0 0))
  (bind _output_get (Variables|Default|SetStartPole _returnvalue))
  (Default|SetAllMaterials _output_get "/Game/Assets/Holograms/M_HologramPlace.M_HologramPlace" false)
  (Default|UpdateCollision _output_get "NoCollision")
  (Utilities|Array|Add (Variables|Default|GetActors%20to%20Ignore) _output_get)
  (|CallParentFunction))

(fn CancelBuild
  (Utilities|FlowControl|Sequence
    (:then_0
      (if (not (Variables|Default|GetStartPlaced))
        (bind _startpole (Variables|Default|GetStartPole)
          (:then
            (Actor|DestroyActor _startpole))
          (:else))))
    (:then_1
      (bind _endpole (Variables|Default|GetEndPole)
        (:then
          (Actor|DestroyActor _endpole))
        (:else)))
    (:then_2
      (|CallParentFunction))))

(fn DestroyBuild
  (params (OutputItems :type Array%20of%20F%20Inventory%20Slot%20Struct%20Structures))
  (Utilities|FlowControl|Sequence
    (:then_0
      (bind _startconnect (Variables|Default|GetStartConnect)
        (:then
          (Default|DisconnectCable _startconnect self))
        (:else)))
    (:then_1
      (bind _endconnect (Variables|Default|GetEndConnect)
        (:then
          (Default|DisconnectCable _endconnect self))
        (:else)))
    (:then_2
      (|CallParentFunction OutputItems)
      (return))))

(fn IsBuildable
  (Utilities|IsStartPlaced
    (:IsPlaced
      (bind _endconnect (Variables|Default|GetEndConnect)
        (:then
          (return (and (Default|CanConnectCable _endconnect) (Default|NoExistingConnection _endconnect (Variables|Default|GetStartConnect)))))
        (:else
          (return (CallFunction|IsBuildable (Variables|Default|GetEndPole))))))
    (:IsNotPlaced
      (bind _startconnect (Variables|Default|GetStartConnect)
        (:then
          (return (Default|CanConnectCable _startconnect)))
        (:else
          (return (CallFunction|IsBuildable (Variables|Default|GetStartPole))))))))