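; BP_Buildings_Merger is a buildable merger building that configures its left and right attach points.
; On BeginPlay it casts the CALeft and CARight child actors to BP_AttachPoint, gives both the same Direction and refreshes each with UpdateSize.
; The parent BeginPlay runs after this setup, and the construction script only calls its parent.
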(event EventBeginPlay
  (for _array_element (Utilities|Array|MakeArray (Variables|Default|GetCA_Left) (Variables|Default|GetCA_Right))
    (bind _asbp_attach_point (Utilities|Casting|CastToBP_AttachPoint (Variables|/Script/Engine.ChildActorComponent|GetChildActor _array_element)))
    (Variables|/Game/Blueprints/Buildings/BP_AttachPoint.BP_AttachPoint_C|SetDirection _asbp_attach_point "NewEnumerator1")
    (Default|UpdateSize _asbp_attach_point (Variables|/Game/Blueprints/Buildings/BP_AttachPoint.BP_AttachPoint_C|GetVectorSize _asbp_attach_point) (Variables|/Game/Blueprints/Buildings/BP_AttachPoint.BP_AttachPoint_C|GetLocationOffset _asbp_attach_point)))
  (|CallParentFunction))

(fn ConstructionScript
  (|CallParentFunction))