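; Tutorial goal building that collects items in an inventory and signals once when the desired item is found there.
; Inventory updates refresh a crafting slot widget showing held versus desired quantity and trigger the one-time reached-desired call.
; Incoming items go into the inventory component, which players open as a HUD container.
; CanOutputItem always returns false with its check disconnected, though StartOutputting can still move stored items to empty connected outputs.
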(event Custom|OnInventoryUpdated
  (bind _bpc_inventorysystem (Variables|Default|GetBPC_InventorySystem))
  (bind _desired (Variables|Default|GetDesired))
  (bind (_success _hasquantity) (Default|QueryforItem _bpc_inventorysystem _desired))
  (CallFunction|UpdateVisuals _hasquantity)
  (if _success
    (Utilities|FlowControl|DoOnce false
      (:Completed
        (Default|CallReachedDesired)))))

(event EventBeginPlay
  (EventDispatchers|BindEventtoOnInventoryUpdated (Variables|Default|GetBPC_InventorySystem) (delegate Custom|OnInventoryUpdated))
  (|CallParentFunction)
  (CallFunction|UpdateVisuals))

(fn ConstructionScript
  (|CallParentFunction)
  (bind _aswb_crafting_item_slot (Utilities|Casting|CastToWB_CraftingItemSlot (UserInterface|GetWidget (Variables|Default|GetWidget))))
  (Variables|Default|SetAs%20WB%20Crafting%20Item%20Slot _aswb_crafting_item_slot)
  (CallFunction|UpdateVisuals))

(fn StartOutputting
  (bind _keys (Utilities|Map|Keys (Variables|Default|GetOutputs)))
  (for _array_element _keys
    (Utilities|IsValid (Variables|/Game/Blueprints/Buildings/BP_AttachPoint.BP_AttachPoint_C|GetConnectedBuild _array_element)
      (:Is%20Valid
        (if (== (.Quantity (Utilities|Struct|BreakFInventorySlotStruct (.Value (Utilities|Map|Find (Variables|Default|GetOutputs) _array_element)))) 0)
          (bind (_success _itemremoved) (Default|RemoveNextItem (Variables|Default|GetBPC_InventorySystem)))
          (if _success
            (CallFunction|ModifyOutputMap _array_element (Utilities|Struct|MakeFInventorySlotStruct _itemremoved 1)))))))
  (|CallParentFunction))

(fn CanInputItem
  (params (InputItem :type DA%20Items%20Object%20Reference))
  (return (Default|CanInputItem (Variables|Default|GetBPC_InventorySystem) (Utilities|Struct|MakeFInventorySlotStruct InputItem 1))))

(fn ModifyInputMap
  (params (Key :type BP%20Attach%20Point%20Object%20Reference) (Value :type F%20Inventory%20Slot%20Struct%20Structure%20%28by%20ref%29))
  (Default|AddtoInventory (Variables|Default|GetBPC_InventorySystem) (.itemdata Value) (.quantity Value))
  (return))

(fn UpdateCollision
  (params (CollisionType :type ECollisionEnabled%20Enum :default "NoCollision"))
  (Collision|SetCollisionEnabled (Variables|Default|GetContainer) CollisionType)
  (|CallParentFunction CollisionType))

(fn Interactwith
  (params (PlayerCharacter :type BP%20Factory%20FPS%20Character%20Object%20Reference))
  (bind (_success _hud) (Default|GetHud PlayerCharacter))
  (if _success
    (Default|OpenMenuContainer _hud (Variables|Default|GetBPC_InventorySystem))
    (return true)
    (else
      (return false))))

(fn CanOutputItem
  (return false))

(fn UpdateVisuals
  (params (Has :type Integer))
  (bind _desired (Variables|Default|GetDesired))
  (Default|UpdateBasicAppearance (Variables|Default|GetAs%20WB%20Crafting%20Item%20Slot) (Utilities|Struct|MakeFInventorySlotStruct (.itemdata _desired) Has) (.quantity _desired)))