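; BP_Buildings_InfiniteSource is a buildable building that acts as an endless supply of a single item, ItemToOutput.
; It always reports that it can output and rejects all input.
; On StartOutputting, it sets every Outputs entry to one ItemToOutput, if valid, then runs the parent's output logic.
; Player interaction is disabled and the hover text is empty.
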(fn ConstructionScript
  (|CallParentFunction))

(fn CanOutputItem
  (return true))

(fn CanInputItem
  (params (InputItem :type DA%20Items%20Object%20Reference))
  (return false))

(fn StartOutputting
  (Utilities|FlowControl|Sequence
    (:then_0
      (Utilities|IsValid (Variables|Default|GetItemToOutput)
        (:Is%20Valid
          (bind _keys (Utilities|Map|Keys (Variables|Default|GetOutputs)))
          (for _array_element _keys
            (Utilities|Map|Add (Variables|Default|GetOutputs) _array_element (Utilities|Struct|MakeFInventorySlotStruct (Variables|Default|GetItemToOutput) 1))))))
    (:then_1
      (|CallParentFunction))))

(fn Interactwith
  (params (PlayerCharacter :type BP%20Factory%20FPS%20Character%20Object%20Reference))
  (return false))

(fn InteractHover
  (return ""))