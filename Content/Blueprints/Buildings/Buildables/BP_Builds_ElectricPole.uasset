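; Buildable electric pole that serves as a cable attachment node, with an interaction that opens the electric network menu.
; An electric node component's cable events update a widget showing attached cables against maximum connections, hidden shortly after each new connection.
; While visible, the widget yaws toward the player camera every tick.
; Connection hover briefly swaps a mesh material to a valid or invalid hologram, reverted by timer.
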(event CableConnected(BSC_ElectricNode)
  (CallFunction|UpdateConnectedWidget)
  (Utilities|FlowControl|Delay 0.2)
  (CallFunction|HideWidget))

(event CableDisconnected(BSC_ElectricNode)
  (CallFunction|UpdateConnectedWidget))

(event EventTick
  (params (DeltaSeconds :type Float%20%28single-precision%29))
  (if (not (Variables|/Script/Engine.SceneComponent|GetbHiddenInGame (Variables|Default|GetWidget)))
    (Transformation|SetWorldRotation (Variables|Default|GetWidget) (Math|Rotator|MakeRotator 0.0 0.0 (.yaw (Math|Rotator|FindLookatRotation (Transformation|GetWorldLocation (Variables|Default|GetWidget)) (Transformation|GetActorLocation (Game|GetPlayerCameraManager 0))))) false false)))

(event EventBeginPlay
  (|CallParentFunction))

(fn ConstructionScript
  (|CallParentFunction))

(fn DisplayWidget
  (Development|SetHiddeninGame (Variables|Default|GetWidget) false false))

(fn HideWidget
  (Development|SetHiddeninGame (Variables|Default|GetWidget) true false))

(fn UpdateConnectedWidget
  (Default|UpdateNumbers (Variables|Default|GetWidgetRef) (Utilities|Set|Length (Variables|/Game/Blueprints/Buildings/BSC_ElectricNode.BSC_ElectricNode_C|GetAttachedCables (Variables|Default|GetBSC_ElectricNode)))))

(fn CreateBuild
  (|CallParentFunction)
  (bind _aswb_pole_cables (Utilities|Casting|CastToWB_PoleCables (UserInterface|GetWidget (Variables|Default|GetWidget))))
  (bind _output_get (Variables|Default|SetWidgetRef _aswb_pole_cables))
  (Default|MakeConnections _output_get (Variables|/Game/Blueprints/Buildings/BSC_ElectricNode.BSC_ElectricNode_C|GetMaxAttachments (Variables|Default|GetBSC_ElectricNode))))

(fn UpdateCollision
  (params (CollisionType :type ECollisionEnabled%20Enum :default "NoCollision"))
  (Collision|SetCollisionEnabled (Variables|Default|GetStaticMesh) CollisionType)
  (|CallParentFunction CollisionType))

(fn FlashConnectHover
  (params (IsBuildable :type Boolean))
  (bind _flashconnecthovertimer (Variables|Default|GetFlashConnectHoverTimer))
  (Rendering|Material|SetMaterial (Variables|Default|GetStaticMesh) 1 (select IsBuildable "/Game/Assets/Holograms/M_HologramPlace.M_HologramPlace" "/Game/Assets/Holograms/M_HologramPlaceInvalid.M_HologramPlaceInvalid"))
  (if (Utilities|Time|IsValidTimerHandle _flashconnecthovertimer)
    (Utilities|Time|ClearandInvalidateTimerbyHandle _flashconnecthovertimer))
  (Utilities|Time|SetTimerbyFunctionName 0 "StopFlashConnectHover" 0.05))

(fn StopFlashConnectHover
  (Rendering|Material|SetMaterial (Variables|Default|GetStaticMesh) 1 "/Game/Assets/Electricity/M_Cable.M_Cable"))

(fn InteractHover
  (return "View Electric Network"))

(fn Interactwith
  (params (PlayerCharacter :type BP%20Factory%20FPS%20Character%20Object%20Reference))
  (bind (_success _hud) (Default|GetHud PlayerCharacter))
  (if _success
    (Default|OpenMenuElectricNetwork _hud (Variables|Default|GetBSC_ElectricNode))
    (return true)
    (else
      (return false))))