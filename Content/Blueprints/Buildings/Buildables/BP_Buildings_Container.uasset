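; Storage container buildable that accepts items into an inventory component, feeds them out to connected builds, and opens a container menu when a player interacts.
; Inputs go straight into the inventory instead of an input map.
; Inventory updates trigger output, rechecked a tick later, moving one item into each empty, connected output slot.
; The output check tests only the first attach point, as its loop returns immediately.
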(event Custom|OnInventoryUpdated
  (if (CallFunction|CanOutputItem)
    (Utilities|FlowControl|DelayUntilNextTick)
    (if (CallFunction|CanOutputItem)
      (CallFunction|StartOutputting))))

(event EventBeginPlay
  (EventDispatchers|BindEventtoOnInventoryUpdated (Variables|Default|GetBPC_InventorySystem) (delegate Custom|OnInventoryUpdated))
  (|CallParentFunction))

(fn ConstructionScript
  (|CallParentFunction))

(fn StartOutputting
  (bind _keys (Utilities|Map|Keys (Variables|Default|GetOutputs)))
  (for _array_element _keys
    (Utilities|IsValid (Variables|/Game/Blueprints/Buildings/BP_AttachPoint.BP_AttachPoint_C|GetConnectedBuild _array_element)
      (:Is%20Valid
        (if (== (.Quantity (Utilities|Struct|BreakFInventorySlotStruct (.Value (Utilities|Map|Find (Variables|Default|GetOutputs) _array_element)))) 0)
          (bind (_success _itemremoved) (Default|RemoveNextItem (Variables|Default|GetBPC_InventorySystem)))
          (if _success
            (CallFunction|ModifyOutputMap _array_element (Utilities|Struct|MakeFInventorySlotStruct _itemremoved 1)))))))
  (|CallParentFunction))

(fn CanInputItem
  (params (InputItem :type DA%20Items%20Object%20Reference))
  (return (Default|CanInputItem (Variables|Default|GetBPC_InventorySystem) (Utilities|Struct|MakeFInventorySlotStruct InputItem 1))))

(fn ModifyInputMap
  (params (Key :type BP%20Attach%20Point%20Object%20Reference) (Value :type F%20Inventory%20Slot%20Struct%20Structure%20%28by%20ref%29))
  (Default|AddtoInventory (Variables|Default|GetBPC_InventorySystem) (.itemdata Value) (.quantity Value))
  (return))

(fn UpdateCollision
  (params (CollisionType :type ECollisionEnabled%20Enum :default "NoCollision"))
  (Collision|SetCollisionEnabled (Variables|Default|GetContainer) CollisionType)
  (|CallParentFunction CollisionType))

(fn Interactwith
  (params (PlayerCharacter :type BP%20Factory%20FPS%20Character%20Object%20Reference))
  (bind (_success _hud) (Default|GetHud PlayerCharacter))
  (if _success
    (Default|OpenMenuContainer _hud (Variables|Default|GetBPC_InventorySystem))
    (return true)
    (else
      (return false))))

(fn CanOutputItem
  (if (Default|IsNotEmpty (Variables|Default|GetBPC_InventorySystem))
    (bind _keys (Utilities|Map|Keys (Variables|Default|GetOutputs)))
    (for _array_element _keys
      (return (CallFunction|CanOutputfromAttachPoint _array_element)))
    (return false)
    (else
      (return false))))