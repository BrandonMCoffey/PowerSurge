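; Building component that makes its owner a node in a cable-linked electricity network, tracking attached cables up to a limit.
; A recursive set-based search gathers connected nodes, totals power consumed and generated, writes capped histories to each and prompts owning buildings to attempt crafting.
; That pass clears the other nodes' looping one-second timers, and connecting a cable starts a new one.
; The latest history sample determines whether energy is sufficient.
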(event EventBeginPlay
  (CallFunction|StartTimer))

(fn DisconnectCable
  (params (Disconnected :type BP%20Builds%20Electric%20Cable%20Object%20Reference))
  (bind _startconnect (Variables|/Game/Blueprints/Buildings/Buildables/BP_Builds_ElectricCable.BP_Builds_ElectricCable_C|GetStartConnect Disconnected))
  (Utilities|FlowControl|Sequence
    (:then_0
      (Utilities|Set|Remove (Variables|Default|GetAttachedCables) Disconnected)
      (Utilities|Set|Remove (Variables|Default|GetConnectedNodes) (select (!= _startconnect self) _startconnect (Variables|/Game/Blueprints/Buildings/Buildables/BP_Builds_ElectricCable.BP_Builds_ElectricCable_C|GetEndConnect Disconnected))))
    (:then_1
      (CallFunction|GetEnergyInformation)
      (Default|CallCableDisconnected))))

(fn ConnectCable
  (params (Cable :type BP%20Builds%20Electric%20Cable%20Object%20Reference))
  (bind _startconnect (Variables|/Game/Blueprints/Buildings/Buildables/BP_Builds_ElectricCable.BP_Builds_ElectricCable_C|GetStartConnect Cable))
  (Utilities|FlowControl|Sequence
    (:then_0
      (Utilities|Set|Add (Variables|Default|GetAttachedCables) Cable)
      (Utilities|Set|Add (Variables|Default|GetConnectedNodes) (select (!= _startconnect self) _startconnect (Variables|/Game/Blueprints/Buildings/Buildables/BP_Builds_ElectricCable.BP_Builds_ElectricCable_C|GetEndConnect Cable))))
    (:then_1
      (CallFunction|StartTimer)
      (Default|CallCableConnected))))

(fn StartTimer
  (bind _returnvalue (Utilities|Time|SetTimerbyEvent (EventDispatchers|CreateEvent :!event GetEnergyInformation) 1.0 true false 1.0))
  (Variables|Default|SetArrayTimer _returnvalue))

(fn GetEnergyInformation
  (bind _allnodes (CallFunction|GetAllConnectedNodes (Utilities|Set|MakeSet self)))
  (bind _result (Utilities|Set|ToArray _allnodes))
  (for _array_element _result
    (LocalVariables|SetLocalTotalConsumption (+ (LocalVariables|GetLocalTotalConsumption) (Variables|BSC_ElectricNode_C|GetPowerConsumed _array_element)))
    (LocalVariables|SetLocalTotalGenerated (+ (LocalVariables|GetLocalTotalGenerated) (Variables|BSC_ElectricNode_C|GetPowerGenerated _array_element))))
  (for _array_element_2 _result
    (CallFunction|UpdateArray _array_element_2 (LocalVariables|GetLocalTotalConsumption) (LocalVariables|GetLocalTotalGenerated))
    (bind _asbp_buildings (Utilities|Casting|CastToBP_Buildings (Components|GetOwner _array_element_2))
      (:then
        (Default|AttemptCrafting _asbp_buildings))
      (:CastFailed
        _))
    (if (!= self _array_element_2)
      (if (Utilities|Time|IsValidTimerHandle (Variables|BSC_ElectricNode_C|GetArrayTimer _array_element_2))
        (Utilities|Time|ClearandInvalidateTimerbyHandle (Variables|BSC_ElectricNode_C|GetArrayTimer _array_element_2)))))
  (return))

(fn CanConnectCable
  (return (< (Utilities|Set|Length (Variables|Default|GetAttachedCables)) (Variables|Default|GetMaxAttachments))))

(fn DestroyLinkedCables
  (bind _result (Utilities|Set|ToArray (Variables|Default|GetAttachedCables)))
  (bind _arrayelement (Utilities|Array|ReverseforEachLoop _result)
    (:LoopBody
      (Default|DestroyBuild _arrayelement))))

(fn HasEnoughEnergy
  (bind _generatedarray (Variables|Default|GetGeneratedArray))
  (bind _consumedarray (Variables|Default|GetConsumedArray))
  (return (< (Utilities|Array|Get(acopy) _consumedarray (Utilities|Array|LastIndex _consumedarray)) (Utilities|Array|Get(acopy) _generatedarray (Utilities|Array|LastIndex _generatedarray)))))

(fn GetAllConnectedNodes
  (params (NodesToIgnore :type Set%20of%20BSC%20Electric%20Node%20Object%20References))
  (bind _result (Utilities|Set|Union (LocalVariables|GetLocalAllNodes) NodesToIgnore))
  (LocalVariables|SetLocalAllNodes _result)
  (bind _result_2 (Utilities|Set|ToArray (Variables|Default|GetConnectedNodes)))
  (for _array_element _result_2
    (if (not (Utilities|Set|Contains NodesToIgnore _array_element))
      (Utilities|Set|Add (LocalVariables|GetLocalAllNodes) _array_element)
      (bind _allnodes (CallFunction|GetAllConnectedNodes _array_element (LocalVariables|GetLocalAllNodes)))
      (LocalVariables|SetLocalAllNodes _allnodes)))
  (return (LocalVariables|GetLocalAllNodes)))

(fn UpdateArray
  (params (Consumed :type Float%20%28double-precision%29) (Generated :type Float%20%28double-precision%29))
  (if (>= (Utilities|Array|Length (Variables|Default|GetGeneratedArray)) (Variables|Default|GetMaxArraySize))
    (Utilities|Array|RemoveIndex (Variables|Default|GetConsumedArray))
    (Utilities|Array|RemoveIndex (Variables|Default|GetGeneratedArray)))
  (Utilities|Array|Add (Variables|Default|GetConsumedArray) Consumed)
  (Utilities|Array|Add (Variables|Default|GetGeneratedArray) Generated))

(fn NoExistingConnection
  (params (Other :type BSC%20Electric%20Node%20Object%20Reference))
  (bind _result (Utilities|Set|Intersection (Variables|BSC_ElectricNode_C|GetAttachedCables Other) (Variables|Default|GetAttachedCables)))
  (return (== (Utilities|Set|Length _result) 0)))