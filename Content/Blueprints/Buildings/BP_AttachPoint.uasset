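; Connection point on buildings that decides whether conveyors can attach, with an Input, Output or NonSpecified direction.
; UpdateSize sizes and offsets the Box, and shows an Arrow rotated and hologram-colored by direction when enabled.
; CanConveyorConnect requires a free point and an incoming direction that is unspecified or different from its own.
; LinkConnectedBuild cross-references both points' parent builds, clearing its own link if its parent is invalid.
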(fn ConstructionScript
  (CallFunction|UpdateSize (Variables|Setup|GetVectorSize) (Variables|Setup|GetLocationOffset))
  (Rendering|Material|SetMaterial (Variables|Default|GetArrow) 0 (Utilities|Select :Index (Variables|Setup|GetDirection) :NewEnumerator0 "/Game/Assets/Holograms/M_HologramNone.M_HologramNone" :NewEnumerator1 "/Game/Assets/Holograms/M_HologramInput.M_HologramInput" :NewEnumerator2 "/Game/Assets/Holograms/M_HologramOutput.M_HologramOutput")))

(fn UpdateSize
  (params (VectorSize :type Vector) (LocationOffset :type Vector))
  (bind _arrow (Variables|Default|GetArrow))
  (bind _box (Variables|Default|GetBox))
  (Variables|Setup|SetVectorSize VectorSize)
  (Variables|Setup|SetLocationOffset LocationOffset)
  (Utilities|FlowControl|Sequence
    (:then_0
      (if (or (Utilities|Enum|Equal(Enum) (Variables|Setup|GetDirection) "NewEnumerator0") (not (Variables|Setup|GetShowArrow)))
        (Development|SetHiddeninGame _arrow true false)
        (else
          (Development|SetHiddeninGame _arrow false false)
          (CallFunction|UpdateArrowColor)
          (Transformation|SetRelativeRotation (Variables|Default|GetArrow) (Math|Rotator|MakeRotator 0.0 0.0 (Utilities|Select :Index (Variables|Setup|GetDirection) :NewEnumerator0 0.0 :NewEnumerator1 1.8e+02 :NewEnumerator2 0.0)) false false))))
    (:then_1
      (Transformation|SetRelativeLocation _box (+ (* (Variables|Setup|GetVectorSize) "1.000000,0.000000,0.000000") (Variables|Setup|GetLocationOffset)) false false)
      (Components|Box|SetBoxExtent _box (Variables|Setup|GetVectorSize) true))))

(fn CanConveyorConnect
  (params (InDirection :type EDirectionEnum%20Enum :default "NewEnumerator0"))
  (if (or (Utilities|Enum|Equal(Enum) InDirection "NewEnumerator0") (Utilities|Enum|NotEqual(Enum) InDirection (Variables|Setup|GetDirection)))
    (return (not (Utilities|IsValid (Variables|Builds|GetConnectedBuild))))
    (else
      (return false))))

(fn LinkConnectedBuild
  (params (OtherAttachPoint :type BP%20Attach%20Point%20Object%20Reference))
  (bind _parentbuild (Variables|BP_AttachPoint_C|GetParentBuild OtherAttachPoint)
    (:then
      (Variables|Builds|SetConnectedBuild _parentbuild)
      (bind _parentbuild_2 (Variables|Builds|GetParentBuild)
        (:then
          (Variables|BP_AttachPoint_C|SetConnectedBuild OtherAttachPoint _parentbuild_2)
          (return true))
        (:else
          (Variables|Builds|SetConnectedBuild 0)
          (return false))))
    (:else
      (return false))))

(fn UpdateArrowColor
  (Rendering|Material|SetMaterial (Variables|Default|GetArrow) 0 (Utilities|Select :Index (Variables|Setup|GetDirection) :NewEnumerator0 "/Game/Assets/Holograms/M_HologramNone.M_HologramNone" :NewEnumerator1 "/Game/Assets/Holograms/M_HologramInput.M_HologramInput" :NewEnumerator2 "/Game/Assets/Holograms/M_HologramOutput.M_HologramOutput")))