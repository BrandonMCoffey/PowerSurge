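; Base actor for placeable buildings, covering preview movement, placement, cancellation and deconstruction, with empty creation and custom-scroll hooks.
; The preview snaps to a grid, yaws in fixed scroll steps, hides far below the world when invalid, and checks buildability with a shrunken bounds box trace.
; Placing restores default mesh materials and enables collision.
; Destroying returns the BuildingData cost items, which also feed the deconstruct info.
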(event EventBeginPlay
  (Placement|CreateBuild))

(fn ConstructionScript)

(fn CreateBuild)

(fn CancelBuild
  (Actor|DestroyActor))

(fn PlaceBuild
  (Update|SetAllMaterials 0 true)
  (Update|UpdateCollision "QueryAndPhysics")
  (return true))

(fn DestroyBuild
  (params (OutputItems :type Array%20of%20F%20Inventory%20Slot%20Struct%20Structures))
  (bind _buildingdata (Variables|Default|GetBuildingData))
  (Utilities|FlowControl|Sequence
    (:then_0
      (Utilities|IsValid _buildingdata
        (:Is%20Valid
          (for _array_element (Variables|/Game/Blueprints/Buildings/DA_Buildable.DA_Buildable_C|GetCost _buildingdata)
            (Utilities|Array|Add OutputItems _array_element)))))
    (:then_1
      (Actor|DestroyActor))))

(fn ScrollBuild
  (params (MouseInput :type Float%20%28double-precision%29))
  (bind _returnvalue (Transformation|GetActorRotation))
  (Transformation|SetActorRotation (Math|Rotator|MakeRotator (.roll _returnvalue) (.pitch _returnvalue) (+ (.yaw _returnvalue) (* MouseInput 45.0)))))

(fn ScrollBuildCustom
  (params (MouseInput :type Float%20%28double-precision%29)))

(fn IsBuildable
  (bind (_origin _boxextent) (Collision|GetActorBounds false true))
  (bind _returnvalue (+ _origin "0.000000,0.000000,20.000000"))
  (if (Variables|Default|GetValidLocation)
    (bind _returnvalue_2 (Collision|BoxTraceByChannel _returnvalue _returnvalue (* _boxextent 0.85) "0, 0, 0" "TraceTypeQuery6" false (Variables|Default|GetActors%20to%20Ignore) "None"))
    (return (not _returnvalue_2))
    (else
      (return false))))

(fn UpdateLocation
  (params (HitInformation :type Hit%20Result%20Structure))
  (Variables|Default|SetValidLocation true)
  (Transformation|SetActorLocation (Class|KismetMathLibrary|VectorSnappedtoGrid (.ImpactPoint (Collision|BreakHitResult HitInformation)) 5e+01) false false))

(fn UpdateLocationInvalid
  (Variables|Default|SetValidLocation false)
  (Transformation|SetActorLocation "0.000000,0.000000,-10000.000000" false false))

(fn SetAllMaterials
  (params (MaterialOverride :type Material%20Interface%20Object%20Reference) (Default :type Boolean))
  (for _array_element (Components|GetChildrenComponents (Variables|Default|GetDefaultSceneRoot) true)
    (bind _asstatic_mesh_component (Utilities|Casting|CastToStaticMeshComponent _array_element))
    (for _index (range 0 (- (Rendering|Material|GetNumMaterials _asstatic_mesh_component) 1))
      (Rendering|Material|SetMaterial _asstatic_mesh_component _index (select Default (Rendering|Material|GetMaterial (Variables|/Script/Engine.StaticMeshComponent|GetStaticMesh _asstatic_mesh_component) _index) MaterialOverride)))))

(fn UpdateCollision
  (params (CollisionType :type ECollisionEnabled%20Enum :default "NoCollision"))
  (if (Utilities|Enum|Equal(Enum) CollisionType "NoCollision")
    (Default|CallDisableCollision)
    (else
      (Default|CallEnableCollision))))

(fn GetDeconstructData
  (bind _buildingdata (Variables|Default|GetBuildingData))
  (return (Utilities|Text|ToText(String) (Utilities|GetClassDisplayName (Utilities|GetClass self))) (select (Utilities|IsValid _buildingdata) (Variables|/Game/Blueprints/Buildings/DA_Buildable.DA_Buildable_C|GetCost _buildingdata) (Utilities|Array|MakeArray))))