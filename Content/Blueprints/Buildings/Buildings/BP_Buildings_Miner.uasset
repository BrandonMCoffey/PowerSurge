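; BP_Buildings_Miner is a placeable mining building that can only be built on a mineral source.
; During placement, UpdateLocation snaps the miner to a hit BP_MineralSource and stores it, otherwise it clears it and defers to the parent.
; IsBuildable requires that stored source, and PlaceBuild copies its recipe and starts crafting before running the parent placement.
; Collision updates also apply to the Container component.
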(event EventBeginPlay
  (|CallParentFunction) ; This node is disabled and will not be called.\nDrag off pins to build functionality.
)

(event Collision|EventActorBeginOverlap
  (params (OtherActor :type Actor%20Object%20Reference)))

(event EventTick
  (params (DeltaSeconds :type Float%20%28single-precision%29)))

(fn ConstructionScript
  (|CallParentFunction))

(fn IsBuildable
  (Variables|Default|GetConnectedMineralSource
    (:then
      (return (|CallParentFunction)))
    (:else
      (return false))))

(fn UpdateLocation
  (params (HitInformation :type Hit%20Result%20Structure))
  (bind _asbp_mineral_source (Utilities|Casting|CastToBP_MineralSource (.HitActor (Collision|BreakHitResult HitInformation)))
    (:then
      (bind _output_get (Variables|Default|SetConnectedMineralSource _asbp_mineral_source))
      (Transformation|SetActorLocation (Transformation|GetActorLocation _output_get) false false))
    (:CastFailed
      (Variables|Default|SetConnectedMineralSource 0)
      (|CallParentFunction HitInformation))))

(fn UpdateCollision
  (params (CollisionType :type ECollisionEnabled%20Enum :default "NoCollision"))
  (Collision|SetCollisionEnabled (Variables|Default|GetContainer) CollisionType)
  (|CallParentFunction CollisionType))

(fn PlaceBuild
  (Utilities|FlowControl|Sequence
    (:then_0
      (bind _connectedmineralsource (Variables|Default|GetConnectedMineralSource)
        (:then
          (CallFunction|ChangeRecipe (Variables|/Game/Blueprints/Buildings/BP_MineralSource.BP_MineralSource_C|GetRecipe _connectedmineralsource))
          (CallFunction|CEStartCrafting))
        (:else)))
    (:then_1
      (bind _success (|CallParentFunction))
      (return _success))))