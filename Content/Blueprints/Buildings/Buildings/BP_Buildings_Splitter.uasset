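; Splitter building that can be placed onto a conveyor belt and distributes incoming items across its outputs.
; During placement it snaps to the belt spline, locks scroll input, allows only straight sections away from belt ends, and splits the belt when built.
; Inputs rotate through available outputs via OutputSwitch, destroying the item actor after handing on its data.
; Attempted inputs are tracked so StartOutputting can restart waiting items.
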(event EventBeginPlay
  (|CallParentFunction) ; This node is disabled and will not be called.\nDrag off pins to build functionality.
)

(event Collision|EventActorBeginOverlap
  (params (OtherActor :type Actor%20Object%20Reference)))

(event EventTick
  (params (DeltaSeconds :type Float%20%28single-precision%29)))

(fn ConstructionScript
  (|CallParentFunction))

(fn PlaceBuild
  (Utilities|FlowControl|Sequence
    (:then_0
      (bind _beltattachedto (Variables|Default|GetBeltAttachedTo)
        (:then
          (Default|SplitBelt _beltattachedto self))
        (:else)))
    (:then_1
      (bind _success (|CallParentFunction))
      (return _success))))

(fn UpdateLocation
  (params (HitInformation :type Hit%20Result%20Structure))
  (bind (_bblockinghit _binitialoverlap _time _distance _location _impactpoint _normal _impactnormal _physmat _hitactor) (Collision|BreakHitResult HitInformation))
  (bind _asbp_builds_belt (Utilities|Casting|CastToBP_Builds_Belt _hitactor)
    (:then
      (Variables|Default|SetBeltAttachedTo _asbp_builds_belt)
      (Transformation|SetActorTransform (|SnapTransformToBelt _impactpoint))
      (Utilities|Array|Add (Variables|Default|GetActors%20to%20Ignore) (Variables|Default|GetBeltAttachedTo)))
    (:CastFailed
      (|CallParentFunction HitInformation)
      (bind _beltattachedto (Variables|Default|GetBeltAttachedTo)
        (:then
          (Utilities|Array|RemoveItem (Variables|Default|GetActors%20to%20Ignore) _beltattachedto)
          (Variables|Default|SetBeltAttachedTo 0))
        (:else)))))

(fn GetInputKeybyLocation
  (params (Belt :type BP%20Builds%20Belt%20Object%20Reference) (WorldLocation :type Vector%20%28by%20ref%29))
  (return (Class|SplineComponent|FindInputKeyClosesttoWorldLocation (Variables|/Game/Blueprints/Buildings/Builds/BP_Builds_Belt.BP_Builds_Belt_C|GetSpline Belt) WorldLocation)))

(fn IsBuildable
  (bind _beltattachedto (Variables|Default|GetBeltAttachedTo))
  (Variables|Default|GetBeltAttachedTo
    (:then
      (bind _output_get (LocalVariables|SetLocalActorDistance (Class|SplineComponent|GetDistanceAlongSplineatSplineInputKey (Variables|/Game/Blueprints/Buildings/Builds/BP_Builds_Belt.BP_Builds_Belt_C|GetSpline _beltattachedto) (CallFunction|GetInputKeybyLocation _beltattachedto (Transformation|GetActorLocation)))))
      (if (|CheckOnEdgeOfBelt _output_get 1.5e+02)
        (return false)
        (else
          (return (|GetOnStraightBeltPath 0.1)))))
    (:else
      (return (|CallParentFunction)))))

(fn ScrollBuild
  (params (MouseInput :type Float%20%28double-precision%29))
  (Variables|Default|GetBeltAttachedTo
    (:then)
    (:else
      (|CallParentFunction MouseInput))))

(fn InputfromAttachPoint
  (params (AttachPoint :type BP%20Attach%20Point%20Object%20Reference) (InputItem :type BP%20Item%20Object%20Reference))
  (bind _itemdata (Variables|/Game/Blueprints/Items/BP_Item.BP_Item_C|GetItemData InputItem))
  (Utilities|Map|Add (Variables|Default|GetAttemptedInputs) AttachPoint InputItem)
  (if (CallFunction|CanOutputItem)
    (Utilities|FlowControl|Sequence
      (:then_0
        (bind _keys (Utilities|Map|Keys (Variables|Default|GetOutputs) :!label _label))
        (if (CallFunction|CanOutputfromAttachPoint (Utilities|Array|Get(acopy) _keys (Variables|Default|GetOutputSwitch)))
          (CallFunction|ModifyOutputMap (Utilities|Array|Get(acopy) _keys (Variables|Default|GetOutputSwitch)) _itemdata)
          (CallFunction|OutputfromAttachPoint (Utilities|Array|Get(acopy) _keys (Variables|Default|GetOutputSwitch)) (Utilities|Struct|BreakFInventorySlotStruct _itemdata))
          (Actor|DestroyActor (.Value (Utilities|Map|Find (Variables|Default|GetAttemptedInputs) AttachPoint)))
          (if (>= (+ (Variables|Default|GetOutputSwitch) 1) (Utilities|Map|Length (Variables|Default|GetOutputs)))
            (Variables|Default|SetOutputSwitch 0)
            (else
              (Variables|Default|SetOutputSwitch (+ (Variables|Default|GetOutputSwitch) 1))))
          (return true)))
      (:then_1
        (for _index (range 0 (- (Utilities|Map|Length (Variables|Default|GetOutputs)) 1))
          (Variables|Default|SetOutputSwitch _index)
          (goto _label))
        (return true)))
    (else
      (return false))))

(fn CanOutputItem
  (bind _keys (Utilities|Map|Keys (Variables|Default|GetOutputs)))
  (for _array_element _keys
    (if (CallFunction|CanOutputfromAttachPoint _array_element)
      (return true)))
  (return false))

(fn StartOutputting
  (bind _keys (Utilities|Map|Keys (Variables|Default|GetAttemptedInputs)))
  (for _array_element _keys
    (Utilities|IsValid (.Value (Utilities|Map|Find (Variables|Default|GetAttemptedInputs) _array_element))
      (:Is%20Valid
        (Default|CERestartMovement (.Value (Utilities|Map|Find (Variables|Default|GetAttemptedInputs) _array_element)))))))