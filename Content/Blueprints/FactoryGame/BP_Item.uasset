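; Item actor for the factory game that rides conveyor belt splines and can be picked up by the player.
; A movement timeline places it by alpha along the belt, stopping when the stopped item ahead is within ItemInterval, even across belts.
; Stop and restart events fire dispatchers that other objects bind to, and a second timeline signals the next spawn.
; At belt end it moves to the next belt or feeds the connected building.
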(event Custom|CE_StopMovement
  (if (CallFunction|ConditiontoStop)
    (Utilities|FlowControl|Sequence
      (:then_0
        (Audio|Components|Audio|Stop (Variables|Default|GetTL_Movement))
        (bind _tl_spawnnext (Variables|Default|GetTL_SpawnNext)
          (:then
            (Audio|Components|Audio|Stop _tl_spawnnext))
          (:else)))
      (:then_1
        (Default|CallTLStopped)))))

(event Custom|CE_ForceStop
  (Utilities|FlowControl|Sequence
    (:then_0
      (Audio|Components|Audio|Stop (Variables|Default|GetTL_Movement))
      (bind _tl_spawnnext (Variables|Default|GetTL_SpawnNext)
        (:then
          (Audio|Components|Audio|Stop _tl_spawnnext))
        (:else)))
    (:then_1
      (Default|CallTLStopped))))

(event Custom|CE_RestartMovement
  (Utilities|FlowControl|Sequence
    (:then_0
      (Audio|Components|Audio|Play (Variables|Default|GetTL_Movement))
      (bind _tl_spawnnext (Variables|Default|GetTL_SpawnNext)
        (:then
          (Audio|Components|Audio|Play _tl_spawnnext))
        (:else)))
    (:then_1
      (Default|CallTLStarted))))

(event Custom|CE_EndOf%20Belt
  (CallFunction|CEForceStop)
  (Variables|Default|SetHasReachedEnd true)
  (bind (_success _out_build _attachpoint) (Default|GetNextBuild (Variables|Default|GetBeltReference)))
  (Utilities|Casting|CastToBP_Builds_Belt _out_build
    (:then
      (Default|ItemMovedtoNextBelt (Variables|Default|GetBeltReference) self))
    (:CastFailed
      (bind _asbp_buildings (Utilities|Casting|CastToBP_Buildings _out_build))
      (Default|InputfromAttachPoint _asbp_buildings _attachpoint self))))

(event EventBeginPlay
  (Components|StaticMesh|SetStaticMesh (Variables|Default|GetStaticMesh) (Variables|/Game/Blueprints/FactoryGame/DA_Items.DA_Items_C|GetStaticMesh (Variables|Default|GetDataAsset)))
  (Variables|Default|GetBeltReference
    (:then
      (Utilities|FlowControl|Sequence
        (:then_0
          (Default|ItemsAddedtoBelt (Variables|Default|GetBeltReference) self true))
        (:then_1
          (CallFunction|SetupTimeline)
          (Components|Timeline|SetPlayRate (Variables|Default|GetTL_SpawnNext) (/ (Variables|Default|GetItemInterval) (Variables|/Game/Blueprints/FactoryGame/BP_Builds_Belt.BP_Builds_Belt_C|GetBeltSpeed (Variables|Default|GetBeltReference))))
          (Utilities|FlowControl|DelayUntilNextTick)
          (Timeline|TL_SpawnNext PlayFromStart
            (:Finished
              (Default|CallSpawnNext)
              (Components|DestroyComponent (Variables|Default|GetTL_SpawnNext)))))))
    (:else)))

(fn ConstructionScript)

(fn ConditiontoStop
  (return (and (CallFunction|IsStopped (Variables|Default|GetItemInFront)) (select (== (Variables|BP_Item_C|GetBeltReference (Variables|Default|GetItemInFront)) (Variables|Default|GetBeltReference)) (< (- (CallFunction|GetDistanceAlongSpline (Variables|Default|GetItemInFront)) (CallFunction|GetDistanceAlongSpline)) (Variables|Default|GetItemInterval)) (< (+ (CallFunction|GetDistanceAlongSpline (Variables|Default|GetItemInFront)) (- (Spline|GetSplineLength (Variables|/Game/Blueprints/FactoryGame/BP_Builds_Belt.BP_Builds_Belt_C|GetSpline (Variables|Default|GetBeltReference))) (CallFunction|GetDistanceAlongSpline))) (Variables|Default|GetItemInterval))))))

(fn BindEvents
  (params (Binding :type BP%20Item%20Object%20Reference))
  (EventDispatchers|BindEventtoTLStopped Binding (EventDispatchers|CreateEvent :!event Custom|CE_StopMovement))
  (EventDispatchers|BindEventtoTLStarted Binding (EventDispatchers|CreateEvent :!event Custom|CE_RestartMovement)))

(fn IsStopped
  (return (not (Audio|Components|Audio|IsPlaying (Variables|Default|GetTL_Movement)))))

(fn IsLastItem
  (return (== (Variables|/Game/Blueprints/FactoryGame/BP_Builds_Belt.BP_Builds_Belt_C|GetLastItemInQueue (Variables|Default|GetBeltReference)) self)))

(fn SetupTimeline
  (params (NewBelt :type BP%20Builds%20Belt%20Object%20Reference))
  (Variables|Default|SetHasReachedEnd false)
  (Utilities|FlowControl|Sequence
    (:then_0
      (bind _newbelt (LocalVariables|GetNewBelt)
        (:then
          (Variables|Default|SetBeltReference _newbelt))
        (:else)))
    (:then_1
      (Components|Timeline|SetPlaybackPosition (Variables|Default|GetTL_Movement) 0.0 false false)
      (Components|Timeline|SetPlayRate (Variables|Default|GetTL_Movement) (|CalculatePlayRate))
      (CallFunction|CERestartMovement))))

(fn GetDistanceAlongSpline
  (return (Default|GetLengthbyAlpha (Variables|Default|GetBeltReference) (Variables|Default|GetAlpha))))

(fn InteractwithActor
  (bind _beltreference (Variables|Default|GetBeltReference)
    (:then
      (Default|ItemPickedUp _beltreference self)
      (bind _asbp_fpsfactory_game_character (Utilities|Casting|CastToBP_FPSFactoryGameCharacter (Game|GetPlayerCharacter 0))
        (:then
          (Default|PickupItem _asbp_fpsfactory_game_character self)
          (return true))
        (:CastFailed
          (return false))))
    (:else
      (return false))))