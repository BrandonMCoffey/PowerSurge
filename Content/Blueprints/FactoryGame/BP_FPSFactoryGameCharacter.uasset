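; First-person factory game character that places and deconstructs builds and interacts with actors via Enhanced Input.
; Hotbar keys spawn a belt or support as a collisionless hologram, yaw-snapped toward the player, which scroll adjusts and Confirm places.
; Looping timers run camera line traces to move the preview or highlight a deconstruct target, which Confirm destroys.
; Builds handle their own placement logic, interaction goes through BPI_Interact, and PickupItem is an empty stub.
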(event Input|EnhancedActionEvents|EnhancedInputActionIA_Scroll
  (params (ActionValue :type Float%20%28double-precision%29) (ElapsedSeconds :type Float%20%28double-precision%29) (TriggeredSeconds :type Float%20%28double-precision%29) (InputAction :type Input%20Action%20Object%20Reference :default "/Game/Blueprints/FactoryGame/Inputs/IA_Scroll.IA_Scroll"))
  (:Started
    (bind _itemtobuild (Variables|Default|GetItemToBuild)
      (:then
        (if (Variables|Default|GetCtrlModifier)
          (Default|ScrollBuildCustom _itemtobuild ActionValue)
          (else
            (Default|ScrollBuild _itemtobuild ActionValue))))
      (:else))))

(event Input|EnhancedActionEvents|EnhancedInputActionIA_CtrlModifier
  (params (ActionValue :type Boolean) (ElapsedSeconds :type Float%20%28double-precision%29) (TriggeredSeconds :type Float%20%28double-precision%29) (InputAction :type Input%20Action%20Object%20Reference :default "/Game/Blueprints/FactoryGame/Inputs/IA_CtrlModifier.IA_CtrlModifier"))
  (:Started
    (Variables|Default|SetCtrlModifier true))
  (:Canceled
    (Variables|Default|SetCtrlModifier false :!label _label))
  (:Completed
    (goto _label)))

(event Input|EnhancedActionEvents|EnhancedInputActionIA_Confirm
  (params (ActionValue :type Boolean) (ElapsedSeconds :type Float%20%28double-precision%29) (TriggeredSeconds :type Float%20%28double-precision%29) (InputAction :type Input%20Action%20Object%20Reference :default "/Game/Blueprints/FactoryGame/Inputs/IA_Confirm.IA_Confirm"))
  (:Started
    (Variables|Default|GetItemToBuild
      (:then
        (CallFunction|PlaceBuild))
      (:else
        (bind _itemtodelete (Variables|Default|GetItemToDelete)
          (:then
            (Default|DestroyBuild _itemtodelete))
          (:else))))))

(event Input|EnhancedActionEvents|EnhancedInputActionIA_Deconstruct
  (params (ActionValue :type Boolean) (ElapsedSeconds :type Float%20%28double-precision%29) (TriggeredSeconds :type Float%20%28double-precision%29) (InputAction :type Input%20Action%20Object%20Reference :default "/Game/Blueprints/FactoryGame/Inputs/IA_Deconstruct.IA_Deconstruct"))
  (:Started
    (if (Utilities|Time|IsValidTimerHandle (Variables|Default|GetDeleteBuild))
      (bind _itemtodelete (Variables|Default|GetItemToDelete)
        (:then
          (Default|SetAllMaterials _itemtodelete 0 true)
          (Variables|Default|SetItemToDelete 0))
        (:else
          _))
      (Utilities|Time|ClearandInvalidateTimerbyHandle (Variables|Default|GetDeleteBuild))
      (else
        (Variables|Default|GetItemToBuild
          (:then
            (CallFunction|CancelBuild))
          (:else
            _))
        (bind _returnvalue (Utilities|Time|SetTimerbyFunctionName 0 "DetermineDelete" 0.05 true))
        (Variables|Default|SetDeleteBuild _returnvalue)))))

(event Input|EnhancedActionEvents|EnhancedInputActionIA_Hotbar1
  (params (ActionValue :type Boolean) (ElapsedSeconds :type Float%20%28double-precision%29) (TriggeredSeconds :type Float%20%28double-precision%29) (InputAction :type Input%20Action%20Object%20Reference :default "/Game/Blueprints/FactoryGame/Inputs/IA_Hotbar1.IA_Hotbar1"))
  (:Started
    (CallFunction|SpawnBuild "/Game/Blueprints/FactoryGame/BP_Builds_BeltSupport.BP_Builds_BeltSupport_C")))

(event Input|EnhancedActionEvents|EnhancedInputActionIA_Hotbar2
  (params (ActionValue :type Boolean) (ElapsedSeconds :type Float%20%28double-precision%29) (TriggeredSeconds :type Float%20%28double-precision%29) (InputAction :type Input%20Action%20Object%20Reference :default "/Game/Blueprints/FactoryGame/Inputs/IA_Hotbar2.IA_Hotbar2"))
  (:Started
    (CallFunction|SpawnBuild "/Game/Blueprints/FactoryGame/BP_Builds_Belt.BP_Builds_Belt_C")))

(event Input|EnhancedActionEvents|EnhancedInputActionIA_Interact
  (params (ActionValue :type Boolean) (ElapsedSeconds :type Float%20%28double-precision%29) (TriggeredSeconds :type Float%20%28double-precision%29) (InputAction :type Input%20Action%20Object%20Reference :default "/Game/Blueprints/FactoryGame/Inputs/IA_Interact.IA_Interact"))
  (:Started
    (bind (_outhit _hitsuccess) (CallFunction|LineTracefromCamera "TraceTypeQuery1"))
    (if _hitsuccess
      (if (Utilities|DoesObjectImplementInterface (.HitActor (Collision|BreakHitResult _outhit)) "/Game/Blueprints/FactoryGame/BPI_Interact.BPI_Interact_C")
        (Class|BPIInteract|InteractwithActor(Message) (.HitActor (Collision|BreakHitResult _outhit)))))))

(event EventBeginPlay
  (Input|AddMappingContext (PlayerController|LocalPlayerSubsystems|GetEnhancedInputLocalPlayerSubsystem (Game|GetPlayerController 0)) "/Game/Blueprints/FactoryGame/Inputs/IMC_FactoryGame.IMC_FactoryGame" 0 "(bIgnoreAllPressedKeysUntilRelease=True,bForceImmediately=False,bNotifyUserSettings=False)"))

(fn ConstructionScript
  (|CallParentFunction))

(fn SpawnBuild
  (params (Class :type BP%20Builds%20Class%20Reference))
  (bind _deletebuild (Variables|Default|GetDeleteBuild))
  (if (Utilities|Time|IsValidTimerHandle _deletebuild)
    (Utilities|Time|ClearandInvalidateTimerbyHandle _deletebuild))
  (bind _itemtobuild (Variables|Default|GetItemToBuild)
    (:then
      (Default|CancelBuild _itemtobuild))
    (:else
      _))
  (bind (_outhit _hitsuccess) (CallFunction|LineTracefromCamera "TraceTypeQuery4"))
  (if _hitsuccess
    (bind _returnvalue (Game|SpawnActorfromClass Class (Math|Transform|MakeTransform (.ImpactPoint (Collision|BreakHitResult _outhit)) (Math|Rotator|MakeRotator 0.0 0.0 (Math|Float|SnapToGrid(Float) (.yaw (Math|Rotator|FindLookatRotation (.ImpactPoint (Collision|BreakHitResult _outhit)) (Transformation|GetActorLocation))) 45.0)) "1.000000,1.000000,1.000000") "Undefined" "MultiplyWithRoot" 0 0 0))
    (bind _output_get (Variables|Default|SetItemToBuild _returnvalue))
    (Default|SetAllMaterials _output_get "/Game/Assets/FactoryAssets/Holograms/M_HologramPlace.M_HologramPlace" false)
    (Default|UpdateCollision _output_get "NoCollision")
    (bind _returnvalue_2 (Utilities|Time|SetTimerbyFunctionName 0 "MovingBuild" 0.05 true))
    (Variables|Default|SetMoveBuild _returnvalue_2)))

(fn MovingBuild
  (bind (_outhit _hitsuccess) (CallFunction|LineTracefromCamera "TraceTypeQuery1"))
  (if _hitsuccess
    (Default|UpdateLocation (Variables|Default|GetItemToBuild) _outhit)))

(fn PlaceBuild
  (if (Default|IsBuildable (Variables|Default|GetItemToBuild))
    (bind _success (Default|PlaceBuild (Variables|Default|GetItemToBuild)))
    (if _success
      (Utilities|Time|ClearandInvalidateTimerbyHandle (Variables|Default|GetMoveBuild))
      (Variables|Default|SetItemToBuild 0))))

(fn CancelBuild
  (bind _itemtobuild (Variables|Default|GetItemToBuild)
    (:then
      (Default|CancelBuild _itemtobuild))
    (:else
      _))
  (Utilities|Time|ClearandInvalidateTimerbyHandle (Variables|Default|GetMoveBuild))
  (Variables|Default|SetItemToBuild 0))

(fn DetermineDelete
  (bind _outhit (CallFunction|LineTracefromCamera "TraceTypeQuery3"))
  (bind _itemtodelete (Variables|Default|GetItemToDelete)
    (:then
      (if (not (== _itemtodelete (.HitActor (Collision|BreakHitResult _outhit))))
        (Default|SetAllMaterials (Variables|Default|GetItemToDelete) 0 true)
        (bind _asbp_builds (Utilities|Casting|CastToBP_Builds (.HitActor (Collision|BreakHitResult _outhit)) :!label _label)
          (:then
            (bind _output_get (Variables|Default|SetItemToDelete _asbp_builds))
            (Default|SetAllMaterials _output_get "/Game/Assets/FactoryAssets/Holograms/M_HologramDeconstruct.M_HologramDeconstruct" false))
          (:CastFailed
            (Variables|Default|SetItemToDelete 0)))))
    (:else
      (goto _label))))

(fn LineTracefromCamera
  (params (TraceChannel :type ETraceTypeQuery%20Enum :default "TraceTypeQuery4"))
  (bind _firstpersoncamera (Variables|Default|GetFirstPersonCamera))
  (bind _returnvalue (Transformation|GetWorldLocation _firstpersoncamera))
  (bind (_outhit _returnvalue_2) (Collision|LineTraceByChannel _returnvalue (+ _returnvalue (* (Math|Vector|GetForwardVector _firstpersoncamera) (Variables|Default|GetBuildRange))) TraceChannel false (Utilities|Array|MakeArray (Variables|Default|GetItemToBuild)) "None"))
  (return _outhit _returnvalue_2))

(fn PickupItem
  (params (New%20Item :type BP%20Item%20Object%20Reference)))