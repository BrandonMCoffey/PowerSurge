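; Base building Blueprint for a factory game, handling item flow between a building's attach points and conveyor belts.
; On BeginPlay it registers itself with child attach points; attaching an output belt records a speed-based interval and calls StartOutputting.
; Output spawns items at belt start when spacing allows, while input checks slot item type and stack limit, and default intake destroys the item.
; Empty or simple default functions serve as hooks for child buildings.
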(event EventBeginPlay
  (|CallParentFunction)
  (for _array_element (Actor|GetAllChildActors true)
    (bind _asbp_attach_point (Utilities|Casting|CastToBP_AttachPoint _array_element))
    (Variables|/Game/Blueprints/FactoryGame/BP_AttachPoint.BP_AttachPoint_C|SetParentBuild _asbp_attach_point self)))

(fn ConstructionScript
  (|CallParentFunction))

(fn BeltAttachedOutput
  (params (AttachPoint :type BP%20Attach%20Point%20Object%20Reference))
  (bind _asbp_builds_belt (Utilities|Casting|CastToBP_Builds_Belt (Variables|/Game/Blueprints/FactoryGame/BP_AttachPoint.BP_AttachPoint_C|GetConnectedBuild AttachPoint))
    (:then
      (Utilities|Map|Add (Variables|Output|GetOutputs) AttachPoint (/ (Variables|Default|GetItemSpawnInterval) (Variables|/Game/Blueprints/FactoryGame/BP_Builds_Belt.BP_Builds_Belt_C|GetBeltSpeed _asbp_builds_belt)))
      (Output|StartOutputting)
      (return))
    (:CastFailed
      (return))))

(fn StartOutputting)

(fn CanOutputItem
  (return true))

(fn OutputfromAttachPoint
  (params (AttachPoint :type BP%20Attach%20Point%20Object%20Reference) (ItemData :type DA%20Items%20Object%20Reference))
  (if (Output|CanOutputItem)
    (bind _asbp_builds_belt (Utilities|Casting|CastToBP_Builds_Belt (Variables|/Game/Blueprints/FactoryGame/BP_AttachPoint.BP_AttachPoint_C|GetConnectedBuild AttachPoint))
      (:then
        (if (Default|CanSpawnNextItem _asbp_builds_belt)
          (bind _returnvalue (Game|SpawnActorfromClass "/Game/Blueprints/FactoryGame/BP_Item.BP_Item_C" (Default|GetTransformbyAlpha _asbp_builds_belt 0.0) "Undefined" "MultiplyWithRoot" 0 ItemData _asbp_builds_belt (Variables|Default|GetItemSpawnInterval) 0))
          (EventDispatchers|BindEventtoSpawnNext _returnvalue (EventDispatchers|CreateEvent :!event StartOutputting))
          (return true)
          (else
            (return false) ; Wrong Spacing Between Items
          )))
      (:CastFailed
        (return false)))
    (else
      (return false))))

(fn ConveyorAttachedInput
  (params (AttachPoint :type BP%20Attach%20Point%20Object%20Reference)))

(fn CanInputItem
  (params (AttachPoint :type BP%20Attach%20Point%20Object%20Reference) (InputItem :type DA%20Items%20Object%20Reference))
  (bind _inputs (Variables|Input|GetInputs))
  (bind (_value _returnvalue) (Utilities|Map|Find _inputs AttachPoint))
  (bind (_itemdata _quantity) (Utilities|Struct|BreakST_InventorySlot _value))
  (if _returnvalue
    (if (== _itemdata InputItem)
      (return (< _quantity (Variables|/Game/Blueprints/FactoryGame/DA_Items.DA_Items_C|GetMaxStack InputItem)))
      (else
        (return false)))))

(fn InputfromAttachPoint
  (params (AttachPoint :type BP%20Attach%20Point%20Object%20Reference) (InputItem :type BP%20Item%20Object%20Reference))
  (Actor|DestroyActor InputItem)
  (return true))

(fn ModifyItemQuantity
  (params (ItemSlot :type ST%20Inventory%20Slot%20Structure%20%28by%20ref%29) (Modifier :type Integer))
  (bind _structout (Utilities|Struct|SetmembersinST_InventorySlot ItemSlot (+ (Utilities|Struct|BreakST_InventorySlot ItemSlot) Modifier)))
  (return _structout))

(fn InteractwithActor
  (return false))