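; A factory container building that stores items in a slot map and passes them on to its outputs, overriding its parent building's input and output logic.
; Input is allowed while slots remain under the maximum; incoming items increment matching incomplete stacks and also add a new slot after the loop.
; Output requires a non-empty storage, drawing from the first slot for each output before calling the parent.
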(fn ConstructionScript
  (|CallParentFunction))

(fn CanOutputItem
  (return (and (|CallParentFunction) (Utilities|Map|IsNotEmpty (Variables|Default|GetStorage)))))

(fn StartOutputting
  (bind _keys (Utilities|Map|Keys (Variables|Default|GetOutputs)))
  (for _array_element _keys
    (bind _keys_2 (Utilities|Map|Keys (Variables|Default|GetStorage)))
    (Utilities|Map|Add (Variables|Default|GetStorage) (Utilities|Array|Get(acopy) _keys_2) (CallFunction|ModifyItemQuantity (.Value (Utilities|Map|Find (Variables|Default|GetStorage) (Utilities|Array|Get(acopy) _keys_2))) -1))
    (Utilities|Map|Add (Variables|Default|GetOutputs) _array_element (Utilities|Struct|MakeFInventorySlotStruct (.ItemData (Utilities|Struct|BreakFInventorySlotStruct (CallFunction|ModifyItemQuantity (.Value (Utilities|Map|Find (Variables|Default|GetStorage) (Utilities|Array|Get(acopy) _keys_2))) -1))) (.quantity (CallFunction|ModifyItemQuantity (.Value (Utilities|Map|Find (Variables|Default|GetOutputs) _array_element)) 1))))
    (if (< (.Quantity (Utilities|Struct|BreakFInventorySlotStruct (CallFunction|ModifyItemQuantity (.Value (Utilities|Map|Find (Variables|Default|GetStorage) (Utilities|Array|Get(acopy) _keys_2))) -1))) 0)
      (Utilities|Map|Remove (Variables|Default|GetStorage) (Utilities|Array|Get(acopy) _keys_2))))
  (|CallParentFunction))

(fn CanInputItem
  (params (InputItem :type DA%20Items%20Object%20Reference))
  (return (< (Utilities|Map|Length (Variables|Default|GetStorage)) (Variables|Default|GetMaxInventorySize))))

(fn ModifyInputMap
  (params (Key :type BP%20Attach%20Point%20Object%20Reference%20%28by%20ref%29) (Value :type F%20Inventory%20Slot%20Struct%20Structure%20%28by%20ref%29))
  (bind _keys (Utilities|Map|Keys (Variables|Default|GetStorage)))
  (for _array_element _keys
    (if (and (CallFunction|IsSlotIncomplete (.Value (Utilities|Map|Find (Variables|Default|GetStorage) _array_element))) (== (Utilities|Struct|BreakFInventorySlotStruct (.Value (Utilities|Map|Find (Variables|Default|GetStorage) _array_element))) (Utilities|Struct|BreakFInventorySlotStruct Value)))
      (Utilities|Map|Add (Variables|Default|GetStorage) _array_element (CallFunction|ModifyItemQuantity (.Value (Utilities|Map|Find (Variables|Default|GetStorage) _array_element)) 1))))
  (Utilities|Map|Add (Variables|Default|GetStorage) (Utilities|Map|Length (Variables|Default|GetStorage)) (Utilities|Struct|MakeFInventorySlotStruct (.itemdata Value) 1))
  (return))