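; Factory building that takes items in through attach points, crafts them by recipe and outputs the results onto conveyor belts.
; BeginPlay sorts child attach points into Input and Output maps, each holding an item slot.
; Incoming items fill slots and start crafting when ingredients and output space allow.
; A timeline scaled to recipe duration times crafting, then inputs are consumed and outputs spawn as BP_Item actors on belts with room.
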(event Custom|CE_StartCrafting
  (Timeline|TL_Crafting PlayFromStart
    (:Finished
      (Crafting|ConsumeInputItems)
      (Crafting|SendCraftedtoOutput)
      (Output|StartOutputting)
      (if (Crafting|CanCraft)
        (CallFunction|CEStartCrafting)))))

(event Custom|CE_ResumeCrafting
  (Timeline|TL_Crafting Play
    (:Finished
      (Crafting|ConsumeInputItems)
      (Crafting|SendCraftedtoOutput)
      (Output|StartOutputting)
      (if (Crafting|CanCraft)
        (CallFunction|CEStartCrafting)))))

(event Custom|CE_StopCrafting
  (Timeline|TL_Crafting Stop
    (:Finished
      (Crafting|ConsumeInputItems)
      (Crafting|SendCraftedtoOutput)
      (Output|StartOutputting)
      (if (Crafting|CanCraft)
        (CallFunction|CEStartCrafting)))))

(event EventBeginPlay
  (|CallParentFunction)
  (for _array_element (Actor|GetAllChildActors true)
    (bind _asbp_attach_point (Utilities|Casting|CastToBP_AttachPoint _array_element))
    (Variables|/Game/Blueprints/FactoryGame/Buildings/BP_AttachPoint.BP_AttachPoint_C|SetParentBuild _asbp_attach_point self)
    (switch Utilities|FlowControl|Switch|SwitchonEDirectionEnum (Variables|/Game/Blueprints/FactoryGame/Buildings/BP_AttachPoint.BP_AttachPoint_C|GetDirection _asbp_attach_point)
      (:NewEnumerator1
        (Utilities|Map|Add :TargetMap (Variables|Input|GetInputs) :Key _asbp_attach_point))
      (:NewEnumerator2
        (Utilities|Map|Add :TargetMap (Variables|Output|GetOutputs) :Key _asbp_attach_point))))
  (Variables|Default|GetRecipe
    (:then
      (Crafting|ChangeRecipe))
    (:else)))

(fn ConstructionScript
  (|CallParentFunction))

(fn BeltAttachedOutput
  (params (AttachPoint :type BP%20Attach%20Point%20Object%20Reference))
  (Utilities|Casting|CastToBP_Builds_Belt (Variables|/Game/Blueprints/FactoryGame/Buildings/BP_AttachPoint.BP_AttachPoint_C|GetConnectedBuild AttachPoint)
    (:then
      (Output|StartOutputting)
      (return))
    (:CastFailed
      (return))))

(fn StartOutputting
  (bind _keys (Utilities|Map|Keys (Variables|Output|GetOutputs)))
  (for _array_element _keys
    (if (> (.Quantity (Utilities|Struct|BreakFInventorySlotStruct (.Value (Utilities|Map|Find (Variables|Output|GetOutputs) _array_element)))) 0)
      (bind _success (Output|OutputfromAttachPoint _array_element (.ItemData (Utilities|Struct|BreakFInventorySlotStruct (.Value (Utilities|Map|Find (Variables|Output|GetOutputs) _array_element))))))
      (if _success
        (Utilities|Map|Add (Variables|Output|GetOutputs) _array_element (Assist|ModifyItemQuantity (.Value (Utilities|Map|Find (Variables|Output|GetOutputs) _array_element)) -1))))))

(fn CanOutputItem
  (return true))

(fn OutputfromAttachPoint
  (params (AttachPoint :type BP%20Attach%20Point%20Object%20Reference) (ItemData :type DA%20Items%20Object%20Reference))
  (if (Output|CanOutputItem)
    (bind _asbp_builds_belt (Utilities|Casting|CastToBP_Builds_Belt (Variables|/Game/Blueprints/FactoryGame/Buildings/BP_AttachPoint.BP_AttachPoint_C|GetConnectedBuild AttachPoint))
      (:then
        (if (Default|CanSpawnNextItem _asbp_builds_belt)
          (bind _returnvalue (Game|SpawnActorfromClass "/Game/Blueprints/FactoryGame/Items/BP_Item.BP_Item_C" (Default|GetTransformbyAlpha _asbp_builds_belt 0.0) "Undefined" "MultiplyWithRoot" 0 ItemData _asbp_builds_belt (Variables|Default|GetItemSpawnInterval) 0))
          (EventDispatchers|BindEventtoSpawnNext _returnvalue (EventDispatchers|CreateEvent :!event StartOutputting))
          (return true)
          (else
            (return false) ; Wrong Spacing Between Items
          )))
      (:CastFailed
        (return false)))
    (else
      (return false))))

(fn ConveyorAttachedInput
  (params (AttachPoint :type BP%20Attach%20Point%20Object%20Reference)))

(fn CanInputItem
  (params (InputItem :type DA%20Items%20Object%20Reference))
  (Variables|Default|GetRecipe
    (:then
      (bind _values (Utilities|Map|Values (Variables|Input|GetInputs)))
      (for _array_element _values
        (Utilities|IsValid (Utilities|Struct|BreakFInventorySlotStruct _array_element)
          (:Is%20Valid
            (if (or (== (.Quantity (Utilities|Struct|BreakFInventorySlotStruct _array_element)) 0) (== (.ItemData (Utilities|Struct|BreakFInventorySlotStruct _array_element)) InputItem))
              (if (Crafting|IsSlotIncomplete _array_element)
                (return true)
                (else
                  (return false)))))
          (:Is%20Not%20Valid
            (for _array_element_2 (Variables|/Game/Blueprints/FactoryGame/Items/DA_Recipe.DA_Recipe_C|GetInputs (Variables|Default|GetRecipe))
              (if (== (Utilities|Struct|BreakFInventorySlotStruct _array_element_2) InputItem)
                (return true)))
            (return false)))))
    (:else
      (return true))))

(fn InputfromAttachPoint
  (params (AttachPoint :type BP%20Attach%20Point%20Object%20Reference) (InputItem :type BP%20Item%20Object%20Reference))
  (if (Input|CanInputItem (Variables|/Game/Blueprints/FactoryGame/Items/BP_Item.BP_Item_C|GetDataAsset InputItem))
    (Utilities|IsValid (Utilities|Struct|BreakFInventorySlotStruct (.Value (Utilities|Map|Find (Variables|Input|GetInputs) AttachPoint)))
      (:Is%20Valid
        (LocalVariables|SetLocalNewStructure (Assist|ModifyItemQuantity (.Value (Utilities|Map|Find (Variables|Input|GetInputs) AttachPoint)) 1)))
      (:Is%20Not%20Valid
        (LocalVariables|SetLocalNewStructure (Utilities|Struct|MakeFInventorySlotStruct (Variables|/Game/Blueprints/FactoryGame/Items/BP_Item.BP_Item_C|GetDataAsset InputItem) 1))))
    (Utilities|FlowControl|Sequence
      (:then_0
        (Crafting|ModifyInputMap AttachPoint (LocalVariables|GetLocalNewStructure))
        (if (Crafting|CanCraft)
          (CallFunction|CEStartCrafting)))
      (:then_1
        (Actor|DestroyActor InputItem)
        (return true)))
    (else
      (return false))))

(fn ModifyItemQuantity
  (params (ItemSlot :type F%20Inventory%20Slot%20Struct%20Structure) (Modifier :type Integer))
  (bind _structout (Utilities|Struct|SetmembersinFInventorySlotStruct ItemSlot (+ (Utilities|Struct|BreakFInventorySlotStruct ItemSlot) Modifier)))
  (return _structout))

(fn IsSlotIncomplete
  (params (Slot :type F%20Inventory%20Slot%20Struct%20Structure))
  (bind (_itemdata _quantity) (Utilities|Struct|BreakFInventorySlotStruct Slot))
  (return (< _quantity (Variables|/Game/Blueprints/FactoryGame/Items/DA_Items.DA_Items_C|GetMaxStack _itemdata))))

(fn ModifyInputMap
  (params (Key :type BP%20Attach%20Point%20Object%20Reference%20%28by%20ref%29) (Value :type F%20Inventory%20Slot%20Struct%20Structure%20%28by%20ref%29))
  (Utilities|Map|Add (Variables|Input|GetInputs) Key Value))

(fn CanCraft
  (Variables|Default|GetRecipe
    (:then
      (if (not (Audio|Components|Audio|IsPlaying (Variables|Default|GetTL_Crafting)))
        (bind _values (Utilities|Map|Values (Variables|Input|GetInputs)))
        (LocalVariables|SetLocalAvailableResources _values)
        (Utilities|FlowControl|Sequence
          (:then_0
            (for _array_element (Variables|/Game/Blueprints/FactoryGame/Items/DA_Recipe.DA_Recipe_C|GetInputs (Variables|Default|GetRecipe))
              (LocalVariables|SetLocalItemRequired (.ItemData (Utilities|Struct|BreakFInventorySlotStruct _array_element)))
              (LocalVariables|SetLocalQuantityRequired (.Quantity (Utilities|Struct|BreakFInventorySlotStruct _array_element)))
              (LocalVariables|SetLocalFoundItem false)
              (bind _array_element_2 (Utilities|Array|ForEachLoopwithBreak (LocalVariables|GetLocalAvailableResources) :!label _label)
                (:LoopBody
                  (if (and (<= (LocalVariables|GetLocalQuantityRequired) (.Quantity (Utilities|Struct|BreakFInventorySlotStruct _array_element_2))) (== (.ItemData (Utilities|Struct|BreakFInventorySlotStruct _array_element_2)) (LocalVariables|GetLocalItemRequired)))
                    (LocalVariables|SetLocalFoundItem true)
                    (goto _label Break)))
                (:Completed
                  (if (not (LocalVariables|GetLocalFoundItem))
                    (return false))))))
          (:then_1
            (bind _values_2 (Utilities|Map|Values (Variables|Output|GetOutputs)))
            (LocalVariables|SetLocalAvailableResources _values_2)
            (for _array_element_3 (Variables|/Game/Blueprints/FactoryGame/Items/DA_Recipe.DA_Recipe_C|GetOutputs (Variables|Default|GetRecipe))
              (LocalVariables|SetLocalItemRequired (.ItemData (Utilities|Struct|BreakFInventorySlotStruct _array_element_3)))
              (LocalVariables|SetLocalQuantityRequired (.Quantity (Utilities|Struct|BreakFInventorySlotStruct _array_element_3)))
              (for _array_element_4 (LocalVariables|GetLocalAvailableResources)
                (if (and (> (+ (LocalVariables|GetLocalQuantityRequired) (.Quantity (Utilities|Struct|BreakFInventorySlotStruct _array_element_4))) (Variables|/Game/Blueprints/FactoryGame/Items/DA_Items.DA_Items_C|GetMaxStack (LocalVariables|GetLocalItemRequired))) (== (.ItemData (Utilities|Struct|BreakFInventorySlotStruct _array_element_4)) (LocalVariables|GetLocalItemRequired)))
                  (return false))))
            (return true)))
        (else
          (return false))))
    (:else
      (return false))))

(fn SendCraftedtoOutput
  (bind _keys (Utilities|Map|Keys (Variables|Output|GetOutputs)))
  (for _array_element _keys
    (for _array_element_2 (Variables|/Game/Blueprints/FactoryGame/Items/DA_Recipe.DA_Recipe_C|GetOutputs (Variables|Default|GetRecipe))
      (if (== (.ItemData (Utilities|Struct|BreakFInventorySlotStruct _array_element_2)) (Utilities|Struct|BreakFInventorySlotStruct (.Value (Utilities|Map|Find (Variables|Output|GetOutputs) _array_element))))
        (LocalVariables|SetLocalQuantityToAdd (.Quantity (Utilities|Struct|BreakFInventorySlotStruct _array_element_2)))))
    (Utilities|Map|Add (Variables|Output|GetOutputs) _array_element (Assist|ModifyItemQuantity (.Value (Utilities|Map|Find (Variables|Output|GetOutputs) _array_element)) (LocalVariables|GetLocalQuantityToAdd)))))

(fn ConsumeInputItems
  (bind _keys (Utilities|Map|Keys (Variables|Input|GetInputs)))
  (for _array_element _keys
    (LocalVariables|SetLocalAttachPoint _array_element)
    (LocalVariables|SetLocalInputItem (.Value (Utilities|Map|Find (Variables|Input|GetInputs) _array_element)))
    (bind _array_element_2 (Utilities|Array|ForEachLoopwithBreak (Variables|/Game/Blueprints/FactoryGame/Items/DA_Recipe.DA_Recipe_C|GetInputs (Variables|Default|GetRecipe)) :!label _label)
      (:LoopBody
        (if (== (.ItemData (Utilities|Struct|BreakFInventorySlotStruct _array_element_2)) (.itemdata (LocalVariables|GetLocalInputItem)))
          (Utilities|Map|Add (Variables|Input|GetInputs) (LocalVariables|GetLocalAttachPoint) (Assist|ModifyItemQuantity (LocalVariables|GetLocalInputItem) (* (.Quantity (Utilities|Struct|BreakFInventorySlotStruct _array_element_2)) -1)))
          (goto _label Break))))))

(fn ChangeRecipe
  (params (Recipe :type DA%20Recipe%20Object%20Reference))
  (Utilities|IsValid Recipe
    (:Is%20Valid
      (Variables|Default|SetRecipe Recipe))
    (:Is%20Not%20Valid
      _))
  (Components|Timeline|SetPlayRate (Variables|Default|GetTL_Crafting) (/ 1.0 (Variables|/Game/Blueprints/FactoryGame/Items/DA_Recipe.DA_Recipe_C|GetDuration (Variables|Default|GetRecipe))))
  (bind _keys (Utilities|Map|Keys (Variables|Output|GetOutputs)))
  (for (_array_element _array_index) _keys
    (Utilities|Map|Add (Variables|Output|GetOutputs) _array_element (Utilities|Struct|MakeFInventorySlotStruct (.itemdata (Utilities|Array|Get(acopy) (Variables|/Game/Blueprints/FactoryGame/Items/DA_Recipe.DA_Recipe_C|GetOutputs (Variables|Default|GetRecipe)) _array_index))))))