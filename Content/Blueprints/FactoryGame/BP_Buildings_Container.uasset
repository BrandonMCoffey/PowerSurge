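; BP_Buildings_Container is a factory building that outputs items from its Storage map through its attach points.
; It extends the parent's CanOutputItem check to also require a non-empty Storage.
; StartOutputting calls the parent, then offers the first stored item to each output attach point.
; Each successful output decrements that slot's quantity by one and removes the entry once it reaches zero.
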(event EventBeginPlay
  (|CallParentFunction) ; This node is disabled and will not be called.\nDrag off pins to build functionality.
)

(event Collision|EventActorBeginOverlap
  (params (OtherActor :type Actor%20Object%20Reference))
  (|CallParentFunction OtherActor) ; This node is disabled and will not be called.\nDrag off pins to build functionality.
)

(event EventTick
  (params (DeltaSeconds :type Float%20%28single-precision%29))
  (|CallParentFunction DeltaSeconds) ; This node is disabled and will not be called.\nDrag off pins to build functionality.
)

(fn ConstructionScript
  (|CallParentFunction))

(fn CanOutputItem
  (return (and (|CallParentFunction) (Utilities|Map|IsNotEmpty (Variables|Default|GetStorage)))))

(fn StartOutputting
  (bind _storage (Variables|Default|GetStorage))
  (|CallParentFunction)
  (bind _keys (Utilities|Map|Keys (Variables|Default|GetOutputs)))
  (for _array_element _keys
    (bind _keys_2 (Utilities|Map|Keys _storage))
    (bind _success (CallFunction|OutputfromAttachPoint _array_element (Utilities|Struct|BreakST_InventorySlot (.Value (Utilities|Map|Find _storage (Utilities|Array|Get(acopy) _keys_2))))))
    (if _success
      (bind _structout (CallFunction|ModifyItemQuantity (.Value (Utilities|Map|Find _storage (Utilities|Array|Get(acopy) _keys_2))) -1))
      (Utilities|Map|Add (Variables|Default|GetStorage) (Utilities|Array|Get(acopy) _keys_2) _structout)
      (if (<= (Utilities|Struct|BreakST_InventorySlot _structout) 0)
        (Utilities|Map|Remove (Variables|Default|GetStorage) (Utilities|Array|Get(acopy) _keys_2))))))