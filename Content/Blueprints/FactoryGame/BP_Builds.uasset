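; BP_Builds is a base actor for placeable buildings, with empty hooks for creation, custom scrolling and collision updates.
; While previewing, it snaps to a 50-unit grid at the hit point, yaws in 45-degree scroll steps, and checks clearance with a slightly shrunken bounds box trace.
; Material overrides apply across child static meshes, and placement restores one default material before requesting full collision; cancelling or destroying removes the actor.
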(event EventBeginPlay
  (Placement|CreateBuild))

(fn ConstructionScript)

(fn CreateBuild)

(fn CancelBuild
  (Actor|DestroyActor))

(fn PlaceBuild
  (Update|SetAllMaterials 0 true)
  (Update|UpdateCollision "QueryAndPhysics")
  (return true))

(fn DestroyBuild
  (Actor|DestroyActor))

(fn ScrollBuild
  (params (MouseInput :type Float%20%28double-precision%29))
  (bind _returnvalue (Transformation|GetActorRotation))
  (Transformation|SetActorRotation (Math|Rotator|MakeRotator (.roll _returnvalue) (.pitch _returnvalue) (+ (.yaw _returnvalue) (* MouseInput 45.0)))))

(fn ScrollBuildCustom
  (params (MouseInput :type Float%20%28double-precision%29)))

(fn IsBuildable
  (bind (_origin _boxextent) (Collision|GetActorBounds false true))
  (bind _returnvalue (Collision|BoxTraceByChannel _origin _origin (* _boxextent 0.9) "0, 0, 0" "TraceTypeQuery4" false (Variables|Default|GetActors%20to%20Ignore) "None"))
  (return (not _returnvalue)))

(fn UpdateLocation
  (params (HitInformation :type Hit%20Result%20Structure))
  (Transformation|SetActorLocation (Class|KismetMathLibrary|VectorSnappedtoGrid (.ImpactPoint (Collision|BreakHitResult HitInformation)) 5e+01) false false))

(fn SetAllMaterials
  (params (MaterialOverride :type Material%20Interface%20Object%20Reference) (Default :type Boolean))
  (for _array_element (Components|GetChildrenComponents (Variables|Default|GetDefaultSceneRoot) true)
    (bind _asstatic_mesh_component (Utilities|Casting|CastToStaticMeshComponent _array_element))
    (for _index (range 0 (- (Rendering|Material|GetNumMaterials _asstatic_mesh_component) 1))
      (Rendering|Material|SetMaterial _asstatic_mesh_component _index (select Default "/Engine/EngineMaterials/DefaultMaterial.DefaultMaterial" MaterialOverride)))))

(fn UpdateCollision
  (params (CollisionType :type ECollisionEnabled%20Enum :default "NoCollision")))