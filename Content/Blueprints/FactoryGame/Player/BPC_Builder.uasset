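; Player builder component that runs build mode: toggles the build overlay and handles previewing, rotating and placing buildings.
; SetToBuild spawns the chosen building as a collision-free hologram, its yaw snapped to 45-degree steps toward the owner.
; While enabled, Tick moves the preview along a camera line trace, and a successful Build spawns the next preview for repeat placement.
; SampleBuilding sphere-traces from the camera to return an existing building's data.
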(event Custom|SetEnabled
  (params (Enabled :type Boolean))
  (bind _overlay (Variables|Default|GetOverlay))
  (bind _output_get (Variables|Default|SetEnabled Enabled))
  (if _output_get
    (UserInterface|Viewport|AddtoViewport _overlay 0)
    (else
      (Widget|RemovefromParent _overlay)
      (Variables|Default|SetToBuildData 0)
      (bind _buildpreview (Variables|Default|GetBuildPreview)
        (:then
          (Default|CancelBuild _buildpreview))
        (:else)))))

(event EventBeginPlay
  (bind _returnvalue (UserInterface|CreateWidget "/Game/Blueprints/UI/Overlays/WB_OverlayBuild.WB_OverlayBuild_C"))
  (Variables|Default|SetOverlay _returnvalue))

(event EventTick
  (params (DeltaSeconds :type Float%20%28single-precision%29))
  (if (Variables|Default|GetEnabled)
    (CallFunction|BuildTrace)))

(fn SampleBuilding
  (bind _returnvalue (Game|GetPlayerCameraManager 0))
  (bind _returnvalue_2 (Transformation|GetActorLocation _returnvalue))
  (bind (_outhit _returnvalue_3) (Collision|SphereTraceByChannel _returnvalue_2 (+ _returnvalue_2 (* (Transformation|GetActorForwardVector _returnvalue) (Variables|Default|GetBuildRange))) 5.0 "TraceTypeQuery4" false 0 "None"))
  (if _returnvalue_3
    (bind _asbp_builds (Utilities|Casting|CastToBP_Builds (.HitActor (Collision|BreakHitResult _outhit)))
      (:then
        (return true (Variables|/Game/Blueprints/FactoryGame/Buildings/BP_Builds.BP_Builds_C|GetBuildingData _asbp_builds)))
      (:CastFailed
        _)))
  (return false 0))

(fn BuildTrace
  (bind (_success _outhit) (CallFunction|LineTrace "TraceTypeQuery1"))
  (if _success
    (Default|UpdateLocation (Variables|Default|GetBuildPreview) _outhit)))

(fn LineTrace
  (params (TraceChannel :type ETraceTypeQuery%20Enum :default "TraceTypeQuery1"))
  (bind _returnvalue (Game|GetPlayerCameraManager 0))
  (bind _returnvalue_2 (Transformation|GetActorLocation _returnvalue))
  (bind (_outhit _returnvalue_3) (Collision|LineTraceByChannel _returnvalue_2 (+ _returnvalue_2 (* (Transformation|GetActorForwardVector _returnvalue) (Variables|Default|GetBuildRange))) TraceChannel false (Utilities|Array|MakeArray (Components|GetOwner)) "None"))
  (if _returnvalue_3
    (return true _outhit)
    (else
      (return false ""))))

(fn Build
  (params (KeyDown :type Boolean))
  (if KeyDown
    (bind _buildpreview (Variables|Default|GetBuildPreview)
      (:then
        (if (Default|IsBuildable _buildpreview)
          (bind _success (Default|PlaceBuild (Variables|Default|GetBuildPreview)))
          (if _success
            (Variables|Default|SetBuildPreview 0)
            (CallFunction|SpawnBuild))))
      (:else))))

(fn SettoBuild
  (params (BuildableID :type DA%20Buildable%20Object%20Reference))
  (bind _output_get (Variables|Default|SetToBuildData BuildableID))
  (Default|SettoBuild (Variables|Default|GetOverlay) _output_get (Variables|Default|GetPlayerInventory))
  (CallFunction|SpawnBuild))

(fn AddRotation
  (params (CustomRot :type Boolean) (MouseInput :type Float%20%28double-precision%29))
  (bind _buildpreview (Variables|Default|GetBuildPreview))
  (if CustomRot
    (Default|ScrollBuildCustom _buildpreview MouseInput)
    (else
      (Default|ScrollBuild _buildpreview MouseInput))))

(fn SpawnBuild
  (bind _buildpreview (Variables|Default|GetBuildPreview)
    (:then
      (Default|CancelBuild _buildpreview))
    (:else
      _))
  (Variables|Default|GetToBuildData
    (:then
      (bind (_success _outhit) (CallFunction|LineTrace "TraceTypeQuery4"))
      (if _success
        (bind _returnvalue (Game|SpawnActorfromClass (Variables|/Game/Blueprints/FactoryGame/Buildings/DA_Buildable.DA_Buildable_C|GetBuildClass (Variables|Default|GetToBuildData)) (Math|Transform|MakeTransform (.ImpactPoint (Collision|BreakHitResult _outhit)) (Math|Rotator|MakeRotator 0.0 0.0 (Math|Float|SnapToGrid(Float) (.yaw (Math|Rotator|FindLookatRotation (.ImpactPoint (Collision|BreakHitResult _outhit)) (Transformation|GetActorLocation (Components|GetOwner)))) 45.0)) "1.000000,1.000000,1.000000") "Undefined" "MultiplyWithRoot" 0 0 0))
        (bind _output_get (Variables|Default|SetBuildPreview _returnvalue))
        (Default|SetAllMaterials _output_get "/Game/Assets/FactoryAssets/Holograms/M_HologramPlace.M_HologramPlace" false)
        (Default|UpdateCollision _output_get "NoCollision")))
    (:else)))