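; BPC_Interaction is a player interaction component that finds what the camera is looking at and lets the player interact with it.
; While enabled, it sphere-traces forward from the camera every tick and caches hit actors implementing BPI_InteractInterface as LookAtActor.
; That actor's look-at message appears in a WB_PopupInteract widget, and Interact forwards the player character to it.
; SetEnabled toggles the widget and clears the target when disabled.
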(event Custom|SetEnabled
  (params (Enabled :type Boolean))
  (bind _displaymessage (Variables|Default|GetDisplayMessage))
  (bind _output_get (Variables|Default|SetEnabled Enabled))
  (if _output_get
    (UserInterface|Viewport|AddtoViewport _displaymessage 0)
    (else
      (Widget|RemovefromParent _displaymessage)
      (Variables|Default|SetLookAtActor 0))))

(event Custom|Interact
  (params (PlayerCharacter :type BP%20Factory%20FPS%20Character%20Object%20Reference))
  (if (Variables|Default|GetEnabled)
    (bind _lookatactor (Variables|Default|GetLookAtActor)
      (:then
        (Class|BPIInteractInterface|Interactwith(Message) _lookatactor PlayerCharacter))
      (:else))))

(event EventTick
  (params (DeltaSeconds :type Float%20%28single-precision%29))
  (if (Variables|Default|GetEnabled)
    (CallFunction|InteractionTrace)))

(event EventBeginPlay
  (bind _returnvalue (UserInterface|CreateWidget "/Game/Blueprints/UI/Popups/WB_PopupInteract.WB_PopupInteract_C"))
  (bind _output_get (Variables|Default|SetDisplayMessage _returnvalue))
  (UserInterface|Viewport|AddtoViewport _output_get 0)
  (Variables|Default|SetEnabled true))

(fn InteractionTrace
  (bind _returnvalue (Game|GetPlayerCameraManager 0))
  (bind _returnvalue_2 (Transformation|GetActorLocation _returnvalue))
  (bind (_outhit _returnvalue_3) (Collision|SphereTraceByChannel _returnvalue_2 (+ _returnvalue_2 (* (Transformation|GetActorForwardVector _returnvalue) (Variables|Default|GetInteractionRange))) 15.0 "TraceTypeQuery1" false 0 "None"))
  (if _returnvalue_3
    (if (!= (Variables|Default|GetLookAtActor) (.HitActor (Collision|BreakHitResult _outhit)))
      (if (Utilities|DoesObjectImplementInterface (.HitActor (Collision|BreakHitResult _outhit)) "/Game/Blueprints/FactoryGame/Inventory/BPI_InteractInterface.BPI_InteractInterface_C")
        (bind _output_get (Variables|Default|SetLookAtActor (.HitActor (Collision|BreakHitResult _outhit))))
        (bind _hudmessage (Class|BPIInteractInterface|Lookat(Message) _output_get))
        (Default|ShowMessage (Variables|Default|GetDisplayMessage) _hudmessage)
        (else
          (Variables|Default|SetLookAtActor 0 :!label _label)
          (Default|ShowMessage (Variables|Default|GetDisplayMessage)))))
    (else
      (goto _label))))