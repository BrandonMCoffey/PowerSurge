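; Player controller for a first-person factory-building game that routes Enhanced Input to the character's interaction, builder and deconstructor components.
; On BeginPlay it adds prioritized mapping contexts, links both build components to the inventory and creates the HUD.
; SetMode switches between Interact, Build and Deconstruct, enabling only the matching component.
; Hotbar keys and building sampling select buildables, while menu, confirm and scroll inputs depend on the current mode.
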(event EventBeginPlay
  (CallFunction|SetupInputMappingContext)
  (CallFunction|SetupVariablesandDependencies)
  (CallFunction|CreateHUDWidget)
  (CallFunction|SetMode "NewEnumerator0"))

(fn ConstructionScript)

(fn SetupInputMappingContext
  (bind _returnvalue (PlayerController|LocalPlayerSubsystems|GetEnhancedInputLocalPlayerSubsystem))
  (Utilities|IsValid _returnvalue
    (:Is%20Valid
      (Input|AddMappingContext _returnvalue "/Game/Blueprints/FactoryGame/Player/Input/IMC_Menus.IMC_Menus" 4 "(bIgnoreAllPressedKeysUntilRelease=True,bForceImmediately=False,bNotifyUserSettings=False)")
      (Input|AddMappingContext _returnvalue "/Game/Blueprints/FactoryGame/Player/Input/IMC_Actions.IMC_Actions" 3 "(bIgnoreAllPressedKeysUntilRelease=True,bForceImmediately=False,bNotifyUserSettings=False)")
      (Input|AddMappingContext _returnvalue "/Game/Blueprints/FactoryGame/Player/Input/IMC_Movement.IMC_Movement" 2 "(bIgnoreAllPressedKeysUntilRelease=True,bForceImmediately=False,bNotifyUserSettings=False)")
      (Input|AddMappingContext _returnvalue "/Game/Blueprints/FactoryGame/Player/Input/IMC_Hotbar.IMC_Hotbar" 1 "(bIgnoreAllPressedKeysUntilRelease=True,bForceImmediately=False,bNotifyUserSettings=False)"))))

(fn CreateHUDWidget
  (if (Pawn|IsLocalPlayerController)
    (bind _returnvalue (UserInterface|CreateWidget "/Game/Blueprints/UI/Menus/WB_PlayerHUD.WB_PlayerHUD_C"))
    (bind _output_get (Variables|Default|SetHUD _returnvalue))
    (UserInterface|Viewport|AddtoViewport _output_get 0)))

(fn SetupVariablesandDependencies
  (bind _output_get (Variables|Default|SetPlayerCharacter (.AsBP%20Factory%20FPSCharacter (Utilities|Casting|CastToBP_FactoryFPSCharacter (Pawn|GetControlledPawn)))))
  (Variables|/Game/Blueprints/FactoryGame/Player/BPC_Builder.BPC_Builder_C|SetPlayerInventory (Variables|/Game/Blueprints/FactoryGame/Player/BP_FactoryFPSCharacter.BP_FactoryFPSCharacter_C|GetBPC_Builder _output_get) (Variables|/Game/Blueprints/FactoryGame/Player/BP_FactoryFPSCharacter.BP_FactoryFPSCharacter_C|GetBPC_InventorySystem _output_get))
  (Variables|/Game/Blueprints/FactoryGame/Player/BPC_Deconstructor.BPC_Deconstructor_C|SetPlayerInventory (Variables|/Game/Blueprints/FactoryGame/Player/BP_FactoryFPSCharacter.BP_FactoryFPSCharacter_C|GetBPC_Deconstructor _output_get) (Variables|/Game/Blueprints/FactoryGame/Player/BP_FactoryFPSCharacter.BP_FactoryFPSCharacter_C|GetBPC_InventorySystem _output_get)))

(fn SwitchtoBuildable
  (params (Buildable :type DA%20Buildable%20Object%20Reference))
  (CallFunction|SetMode "NewEnumerator1")
  (Default|SettoBuild (Variables|/Game/Blueprints/FactoryGame/Player/BP_FactoryFPSCharacter.BP_FactoryFPSCharacter_C|GetBPC_Builder (Variables|Default|GetPlayerCharacter)) Buildable))

(event Custom|SetMode
  (params (Selection :type EInteractMode%20Enum :default "NewEnumerator0"))
  (if (Utilities|Enum|NotEqual(Enum) Selection (Variables|Default|GetMode))
    (bind _output_get (Variables|Default|SetMode Selection))
    (Default|SetEnabled (Variables|/Game/Blueprints/FactoryGame/Player/BP_FactoryFPSCharacter.BP_FactoryFPSCharacter_C|GetBPC_Interaction (Variables|Default|GetPlayerCharacter)) (Utilities|Enum|Equal(Enum) _output_get "NewEnumerator0"))
    (Default|SetEnabled (Variables|/Game/Blueprints/FactoryGame/Player/BP_FactoryFPSCharacter.BP_FactoryFPSCharacter_C|GetBPC_Builder (Variables|Default|GetPlayerCharacter)) (Utilities|Enum|Equal(Enum) _output_get "NewEnumerator1"))
    (Default|SetEnabled (Variables|/Game/Blueprints/FactoryGame/Player/BP_FactoryFPSCharacter.BP_FactoryFPSCharacter_C|GetBPC_Deconstructor (Variables|Default|GetPlayerCharacter)) (Utilities|Enum|Equal(Enum) _output_get "NewEnumerator2"))
    (if (not (Utilities|Enum|Equal(Enum) _output_get "NewEnumerator1"))
      (Default|SelectIndex (Variables|/Game/Blueprints/UI/Menus/WB_PlayerHUD.WB_PlayerHUD_C|GetWB_Hotbar (Variables|Default|GetHUD)) -1))))

(event Input|EnhancedActionEvents|EnhancedInputActionIA_OpenMenuInventory
  (params (ActionValue :type Boolean) (ElapsedSeconds :type Float%20%28double-precision%29) (TriggeredSeconds :type Float%20%28double-precision%29) (InputAction :type Input%20Action%20Object%20Reference :default "/Game/Blueprints/FactoryGame/Player/Input/InputsMenus/IA_OpenMenuInventory.IA_OpenMenuInventory"))
  (:Started
    (CallFunction|SetMode "NewEnumerator0")
    (Default|OpenMenuInventory (Variables|Default|GetHUD))))

(event Input|EnhancedActionEvents|EnhancedInputActionIA_OpenMenuPause
  (params (ActionValue :type Boolean) (ElapsedSeconds :type Float%20%28double-precision%29) (TriggeredSeconds :type Float%20%28double-precision%29) (InputAction :type Input%20Action%20Object%20Reference :default "/Game/Blueprints/FactoryGame/Player/Input/InputsMenus/IA_OpenMenuPause.IA_OpenMenuPause"))
  (:Started
    (if (Utilities|Enum|Equal(Enum) (Variables|Default|GetMode) "NewEnumerator0")
      (Default|OpenMenuPause (Variables|Default|GetHUD))
      (else
        (CallFunction|SetMode "NewEnumerator0")))))

(event Input|EnhancedActionEvents|EnhancedInputActionIA_OpenMenuBuild
  (params (ActionValue :type Boolean) (ElapsedSeconds :type Float%20%28double-precision%29) (TriggeredSeconds :type Float%20%28double-precision%29) (InputAction :type Input%20Action%20Object%20Reference :default "/Game/Blueprints/FactoryGame/Player/Input/InputsMenus/IA_OpenMenuBuild.IA_OpenMenuBuild"))
  (:Started
    (if (Utilities|Enum|Equal(Enum) (Variables|Default|GetMode) "NewEnumerator0")
      (Default|OpenMenuBuild (Variables|Default|GetHUD))
      (else
        (CallFunction|SetMode "NewEnumerator0")))))

(event Input|EnhancedActionEvents|EnhancedInputActionIA_Interact
  (params (ActionValue :type Boolean) (ElapsedSeconds :type Float%20%28double-precision%29) (TriggeredSeconds :type Float%20%28double-precision%29) (InputAction :type Input%20Action%20Object%20Reference :default "/Game/Blueprints/FactoryGame/Player/Input/InputsActions/IA_Interact.IA_Interact"))
  (bind _playercharacter (Variables|Default|GetPlayerCharacter))
  (:Started
    (Default|Interact (Variables|/Game/Blueprints/FactoryGame/Player/BP_FactoryFPSCharacter.BP_FactoryFPSCharacter_C|GetBPC_Interaction _playercharacter) _playercharacter)))

(event Input|EnhancedActionEvents|EnhancedInputActionIA_Scroll
  (params (ActionValue :type Float%20%28double-precision%29) (ElapsedSeconds :type Float%20%28double-precision%29) (TriggeredSeconds :type Float%20%28double-precision%29) (InputAction :type Input%20Action%20Object%20Reference :default "/Game/Blueprints/FactoryGame/Player/Input/InputsActions/IA_Scroll.IA_Scroll"))
  (switch Utilities|FlowControl|Switch|SwitchonEInteractMode (Variables|Default|GetMode)
    (:NewEnumerator1
      (Default|AddRotation (Variables|/Game/Blueprints/FactoryGame/Player/BP_FactoryFPSCharacter.BP_FactoryFPSCharacter_C|GetBPC_Builder (Variables|Default|GetPlayerCharacter)) (Variables|Default|GetCtrlModifier) ActionValue))))

(event Input|EnhancedActionEvents|EnhancedInputActionIA_SampleBuilding
  (params (ActionValue :type Boolean) (ElapsedSeconds :type Float%20%28double-precision%29) (TriggeredSeconds :type Float%20%28double-precision%29) (InputAction :type Input%20Action%20Object%20Reference :default "/Game/Blueprints/FactoryGame/Player/Input/InputsActions/IA_SampleBuilding.IA_SampleBuilding"))
  (bind _playercharacter (Variables|Default|GetPlayerCharacter))
  (bind _bpc_builder (Variables|/Game/Blueprints/FactoryGame/Player/BP_FactoryFPSCharacter.BP_FactoryFPSCharacter_C|GetBPC_Builder _playercharacter))
  (bind (_success _buildableid) (Default|SampleBuilding _bpc_builder))
  (:Started
    (if _success
      (CallFunction|SwitchtoBuildable _buildableid))))

(event Input|EnhancedActionEvents|EnhancedInputActionIA_ToggleDeconstructor
  (params (ActionValue :type Boolean) (ElapsedSeconds :type Float%20%28double-precision%29) (TriggeredSeconds :type Float%20%28double-precision%29) (InputAction :type Input%20Action%20Object%20Reference :default "/Game/Blueprints/FactoryGame/Player/Input/InputsActions/IA_ToggleDeconstructor.IA_ToggleDeconstructor"))
  (:Started
    (switch Utilities|FlowControl|Switch|SwitchonEInteractMode (Variables|Default|GetMode)
      (:NewEnumerator0
        (CallFunction|SetMode "NewEnumerator2" :!label _label))
      (:NewEnumerator1
        (goto _label))
      (:NewEnumerator2
        (CallFunction|SetMode "NewEnumerator0")))))

(event Input|EnhancedActionEvents|EnhancedInputActionIA_CtrlModifier
  (params (ActionValue :type Boolean) (ElapsedSeconds :type Float%20%28double-precision%29) (TriggeredSeconds :type Float%20%28double-precision%29) (InputAction :type Input%20Action%20Object%20Reference :default "/Game/Blueprints/FactoryGame/Player/Input/InputsActions/IA_CtrlModifier.IA_CtrlModifier"))
  (Variables|Default|SetCtrlModifier ActionValue))

(event Input|EnhancedActionEvents|EnhancedInputActionIA_ConfirmAction
  (params (ActionValue :type Boolean) (ElapsedSeconds :type Float%20%28double-precision%29) (TriggeredSeconds :type Float%20%28double-precision%29) (InputAction :type Input%20Action%20Object%20Reference :default "/Game/Blueprints/FactoryGame/Player/Input/InputsActions/IA_ConfirmAction.IA_ConfirmAction"))
  (:Started
    (switch Utilities|FlowControl|Switch|SwitchonEInteractMode (Variables|Default|GetMode) :!label _label
      (:NewEnumerator1
        (Default|Build (Variables|/Game/Blueprints/FactoryGame/Player/BP_FactoryFPSCharacter.BP_FactoryFPSCharacter_C|GetBPC_Builder (Variables|Default|GetPlayerCharacter)) ActionValue))
      (:NewEnumerator2
        (Default|Deconstruct (Variables|/Game/Blueprints/FactoryGame/Player/BP_FactoryFPSCharacter.BP_FactoryFPSCharacter_C|GetBPC_Deconstructor (Variables|Default|GetPlayerCharacter)) ActionValue))))
  (:Completed
    (goto _label)))

(event Custom|ActionHotbar
  (params (Index :type Integer))
  (bind _hud (Variables|Default|GetHUD))
  (bind _wb_hotbar (Variables|/Game/Blueprints/UI/Menus/WB_PlayerHUD.WB_PlayerHUD_C|GetWB_Hotbar _hud))
  (bind _buildableid (Default|SelectIndex _wb_hotbar Index))
  (Utilities|IsValid _buildableid
    (:Is%20Valid
      (CallFunction|SwitchtoBuildable _buildableid))
    (:Is%20Not%20Valid
      (Default|SelectIndex _wb_hotbar -1)
      (CallFunction|SetMode "NewEnumerator0"))))

(event Input|EnhancedActionEvents|EnhancedInputActionIA_Hotbar1
  (params (ActionValue :type Boolean) (ElapsedSeconds :type Float%20%28double-precision%29) (TriggeredSeconds :type Float%20%28double-precision%29) (InputAction :type Input%20Action%20Object%20Reference :default "/Game/Blueprints/FactoryGame/Player/Input/InputsHotbar/IA_Hotbar1.IA_Hotbar1"))
  (:Started
    (CallFunction|ActionHotbar 1)))

(event Input|EnhancedActionEvents|EnhancedInputActionIA_Hotbar2
  (params (ActionValue :type Boolean) (ElapsedSeconds :type Float%20%28double-precision%29) (TriggeredSeconds :type Float%20%28double-precision%29) (InputAction :type Input%20Action%20Object%20Reference :default "/Game/Blueprints/FactoryGame/Player/Input/InputsHotbar/IA_Hotbar2.IA_Hotbar2"))
  (:Started
    (CallFunction|ActionHotbar 2)))

(event Input|EnhancedActionEvents|EnhancedInputActionIA_Hotbar0
  (params (ActionValue :type Boolean) (ElapsedSeconds :type Float%20%28double-precision%29) (TriggeredSeconds :type Float%20%28double-precision%29) (InputAction :type Input%20Action%20Object%20Reference :default "/Game/Blueprints/FactoryGame/Player/Input/InputsHotbar/IA_Hotbar0.IA_Hotbar0"))
  (:Started
    (CallFunction|ActionHotbar)))

(event Input|EnhancedActionEvents|EnhancedInputActionIA_Hotbar3
  (params (ActionValue :type Boolean) (ElapsedSeconds :type Float%20%28double-precision%29) (TriggeredSeconds :type Float%20%28double-precision%29) (InputAction :type Input%20Action%20Object%20Reference :default "/Game/Blueprints/FactoryGame/Player/Input/InputsHotbar/IA_Hotbar3.IA_Hotbar3"))
  (:Started
    (CallFunction|ActionHotbar 3)))

(event Input|EnhancedActionEvents|EnhancedInputActionIA_Hotbar4
  (params (ActionValue :type Boolean) (ElapsedSeconds :type Float%20%28double-precision%29) (TriggeredSeconds :type Float%20%28double-precision%29) (InputAction :type Input%20Action%20Object%20Reference :default "/Game/Blueprints/FactoryGame/Player/Input/InputsHotbar/IA_Hotbar4.IA_Hotbar4"))
  (:Started
    (CallFunction|ActionHotbar 4)))

(event Input|EnhancedActionEvents|EnhancedInputActionIA_Hotbar5
  (params (ActionValue :type Boolean) (ElapsedSeconds :type Float%20%28double-precision%29) (TriggeredSeconds :type Float%20%28double-precision%29) (InputAction :type Input%20Action%20Object%20Reference :default "/Game/Blueprints/FactoryGame/Player/Input/InputsHotbar/IA_Hotbar5.IA_Hotbar5"))
  (:Started
    (CallFunction|ActionHotbar 5)))

(event Input|EnhancedActionEvents|EnhancedInputActionIA_Hotbar6
  (params (ActionValue :type Boolean) (ElapsedSeconds :type Float%20%28double-precision%29) (TriggeredSeconds :type Float%20%28double-precision%29) (InputAction :type Input%20Action%20Object%20Reference :default "/Game/Blueprints/FactoryGame/Player/Input/InputsHotbar/IA_Hotbar6.IA_Hotbar6"))
  (:Started
    (CallFunction|ActionHotbar 6)))

(event Input|EnhancedActionEvents|EnhancedInputActionIA_Hotbar7
  (params (ActionValue :type Boolean) (ElapsedSeconds :type Float%20%28double-precision%29) (TriggeredSeconds :type Float%20%28double-precision%29) (InputAction :type Input%20Action%20Object%20Reference :default "/Game/Blueprints/FactoryGame/Player/Input/InputsHotbar/IA_Hotbar7.IA_Hotbar7"))
  (:Started
    (CallFunction|ActionHotbar 7)))

(event Input|EnhancedActionEvents|EnhancedInputActionIA_Hotbar8
  (params (ActionValue :type Boolean) (ElapsedSeconds :type Float%20%28double-precision%29) (TriggeredSeconds :type Float%20%28double-precision%29) (InputAction :type Input%20Action%20Object%20Reference :default "/Game/Blueprints/FactoryGame/Player/Input/InputsHotbar/IA_Hotbar8.IA_Hotbar8"))
  (:Started
    (CallFunction|ActionHotbar 8)))

(event Input|EnhancedActionEvents|EnhancedInputActionIA_Hotbar9
  (params (ActionValue :type Boolean) (ElapsedSeconds :type Float%20%28double-precision%29) (TriggeredSeconds :type Float%20%28double-precision%29) (InputAction :type Input%20Action%20Object%20Reference :default "/Game/Blueprints/FactoryGame/Player/Input/InputsHotbar/IA_Hotbar9.IA_Hotbar9"))
  (:Started
    (CallFunction|ActionHotbar 9)))