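; BP_Builds_BeltSupport is a placeable factory build for a conveyor belt support with adjustable height, extending a parent build Blueprint.
; Scroll input changes the height override in clamped steps and rebuilds the meshes.
; At zero height it shows a single support mesh; above that it reveals the base, stacks instanced middle segments and raises a separate top mesh.
; Collision updates apply to all three parts.
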(fn ConstructionScript
  (|CallParentFunction))

(fn CreateBuild
  (|CallParentFunction)
  (CallFunction|StaticMeshbyHeight))

(fn PlaceBuild
  (bind _success (|CallParentFunction))
  (return _success))

(fn ScrollBuildCustom
  (params (MouseInput :type Float%20%28double-precision%29))
  (Variables|Default|SetHeightOverride (Math|Float|Clamp(Float) (+ (* MouseInput 5e+01) (Variables|Default|GetHeightOverride)) 0.0 1.5e+02))
  (CallFunction|StaticMeshbyHeight))

(fn StaticMeshbyHeight
  (Components|InstancedStaticMesh|ClearInstances (Variables|Default|GetISM_Mid))
  (if (== (Variables|Default|GetHeightOverride) 0.0)
    (Transformation|SetRelativeLocation (Variables|Default|GetTop) "0, 0, 0" false false)
    (Development|SetHiddeninGame (Variables|Default|GetBase) true false)
    (Components|StaticMesh|SetStaticMesh (Variables|Default|GetTop) "/Game/Assets/FactoryAssets/BeltSupport/SM_BeltSupport.SM_BeltSupport")
    (else
      (Development|SetHiddeninGame (Variables|Default|GetBase) false false)
      (for _index (range 0 (- (Math|Float|Truncate (/ (Variables|Default|GetHeightOverride) 5e+01)) 1))
        (switch int _index
          (:Default
            (Components|InstancedStaticMesh|AddInstance (Variables|Default|GetISM_Mid) (Math|Transform|MakeTransform (* _index "0.000000,0.000000,50.000000") "0, 0, 0" "1.000000,1.000000,1.000000") false))))
      (Components|StaticMesh|SetStaticMesh (Variables|Default|GetTop) "/Game/Assets/FactoryAssets/BeltSupport/SM_BeltSupport_Top.SM_BeltSupport_Top")
      (Transformation|SetRelativeLocation (Variables|Default|GetTop) (Math|Vector|MakeVector 0.0 0.0 (Variables|Default|GetHeightOverride)) false false))))

(fn UpdateCollision
  (params (CollisionType :type ECollisionEnabled%20Enum :default "NoCollision"))
  (|CallParentFunction CollisionType)
  (Collision|SetCollisionEnabled (Variables|Default|GetTop) CollisionType))