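; Player component for a deconstruct mode that removes placed builds and returns their items to the inventory.
; While enabled and not deconstructing, Tick sphere-traces from the camera, giving the targeted BP_Builds a hologram material and naming it on an overlay widget.
; Holding the key runs a timer shown as overlay progress; on completion the build is destroyed and its merged item stacks are added to PlayerInventory.
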(event Custom|SetEnabled
  (params (Enabled :type Boolean))
  (bind _overlay (Variables|Default|GetOverlay))
  (bind _output_get (Variables|Default|SetEnabled Enabled))
  (if _output_get
    (UserInterface|Viewport|AddtoViewport _overlay 0)
    (else
      (Widget|RemovefromParent _overlay)
      (Variables|Default|SetDeconstructing false)
      (bind _todeconstruct (Variables|Default|GetToDeconstruct)
        (:then
          (Default|SetAllMaterials _todeconstruct 0 true)
          (Variables|Default|SetToDeconstruct 0))
        (:else)))))

(event Custom|Deconstruct
  (params (KeyDown :type Boolean))
  (if KeyDown
    (Variables|Default|GetToDeconstruct
      (:then
        (Variables|Default|SetDeconstructing true))
      (:else
        (Variables|Default|SetDeconstructing false :!label _label)))
    (else
      (goto _label)))
  (Variables|Default|SetTimer 0.0)
  (Default|SetDeconstructPercent (Variables|Default|GetOverlay) 0.0))

(event EventBeginPlay
  (bind _returnvalue (UserInterface|CreateWidget "/Game/Blueprints/UI/Overlays/WB_OverlayDeconstructor.WB_OverlayDeconstructor_C"))
  (Variables|Default|SetOverlay _returnvalue))

(event EventTick
  (params (DeltaSeconds :type Float%20%28single-precision%29))
  (if (Variables|Default|GetEnabled)
    (if (Variables|Default|GetDeconstructing)
      (bind _output_get (Variables|Default|SetTimer (+ (Variables|Default|GetTimer) DeltaSeconds)))
      (Default|SetDeconstructPercent (Variables|Default|GetOverlay) (/ _output_get (Variables|Default|GetTimeToDeconstruct)))
      (if (>= _output_get (Variables|Default|GetTimeToDeconstruct))
        (CallFunction|DeconstructActor))
      (else
        (CallFunction|DeconstructTrace)))))

(fn DeconstructTrace
  (bind _returnvalue (Game|GetPlayerCameraManager 0))
  (bind _returnvalue_2 (Transformation|GetActorLocation _returnvalue))
  (bind (_outhit _returnvalue_3) (Collision|SphereTraceByChannel _returnvalue_2 (+ _returnvalue_2 (* (Transformation|GetActorForwardVector _returnvalue) (Variables|Default|GetDeconstructRange))) 5.0 "TraceTypeQuery3" false 0 "None"))
  (if _returnvalue_3
    (if (!= (Variables|Default|GetToDeconstruct) (.HitActor (Collision|BreakHitResult _outhit)))
      (bind _todeconstruct (Variables|Default|GetToDeconstruct)
        (:then
          (Default|SetAllMaterials _todeconstruct 0 true))
        (:else
          _))
      (Default|ResettoDeconstruct (Variables|Default|GetOverlay))
      (bind _asbp_builds (Utilities|Casting|CastToBP_Builds (.HitActor (Collision|BreakHitResult _outhit))))
      (bind _output_get (Variables|Default|SetToDeconstruct _asbp_builds))
      (Default|SetAllMaterials _output_get "/Game/Assets/Holograms/M_HologramDeconstruct.M_HologramDeconstruct" false)
      (Default|SettoDeconstruct (Variables|Default|GetOverlay) (.Name (Default|GetDeconstructData _output_get))))
    (else
      (bind _todeconstruct_2 (Variables|Default|GetToDeconstruct)
        (:then
          (Default|SetAllMaterials _todeconstruct_2 0 true)
          (Variables|Default|SetToDeconstruct 0)
          (Default|ResettoDeconstruct (Variables|Default|GetOverlay)))
        (:else)))))

(fn DeconstructActor
  (bind _todeconstruct (Variables|Default|GetToDeconstruct)
    (:then
      (bind _output_get (LocalVariables|SetOutputItems (Utilities|Array|MakeArray)))
      (Default|DestroyBuild _todeconstruct _output_get)
      (Utilities|FlowControl|Sequence
        (:then_0
          (bind _output (CallFunction|CombineDuplicateItems (LocalVariables|GetOutputItems)))
          (for _array_element _output
            (Default|AddtoInventory (Variables|Default|GetPlayerInventory) (.ItemData (Utilities|Struct|BreakFInventorySlotStruct _array_element)) (.Quantity (Utilities|Struct|BreakFInventorySlotStruct _array_element)))
            (Development|PrintString (Utilities|String|Append (Utilities|String|ToString(Integer) (.Quantity (Utilities|Struct|BreakFInventorySlotStruct _array_element))) (Utilities|GetDisplayName (.ItemData (Utilities|Struct|BreakFInventorySlotStruct _array_element)))))))
        (:then_1
          (Variables|Default|SetDeconstructing false)
          (Variables|Default|SetToDeconstruct 0)
          (Default|ResettoDeconstruct (Variables|Default|GetOverlay)))))
    (:else)))