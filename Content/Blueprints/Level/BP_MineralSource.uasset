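; BP_MineralSource is an interactable mineral source that gives the player items when mined.
; Its hover prompt reads "Mine" plus the item name from the first output of its Recipe.
; Interacting adds that output's item and quantity to the player's BPCInventorySystem and returns whether the add succeeded.
; The graphs shown contain no depletion, cooldown or recipe input check.
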(fn ConstructionScript)

(fn InteractHover
  (return (Utilities|Text|FormatText "Mine {Mineral}" (Variables|/Game/Blueprints/Items/DA_Items.DA_Items_C|GetName (.itemdata (Default|FirstOutput (Variables|Default|GetRecipe)))))))

(fn Interactwith
  (params (PlayerCharacter :type BP%20Factory%20FPS%20Character%20Object%20Reference))
  (bind _recipe (Variables|Default|GetRecipe))
  (bind _output (Default|FirstOutput _recipe))
  (bind _success (Default|AddtoInventory (Variables|/Game/Blueprints/Player/BP_FactoryFPSCharacter.BP_FactoryFPSCharacter_C|GetBPC_InventorySystem PlayerCharacter) (.itemdata _output) (.quantity _output)))
  (return _success))