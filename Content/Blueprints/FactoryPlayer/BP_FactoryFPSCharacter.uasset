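; BP_FactoryFPSCharacter is the player character for the factory game, driven by Enhanced Input actions for look, move, jump and sprint.
; Sprint plays and reverses a Timeline that blends max walk speed between walking and running.
; On BeginPlay it loads the inventory component from player data stored in the GameInstance.
; GetHud fetches the HUD from the factory player controller, while RefreshInputs is an empty stub.
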(event Input|EnhancedActionEvents|EnhancedInputActionIA_Sprint
  (params (ActionValue :type Boolean) (ElapsedSeconds :type Float%20%28double-precision%29) (TriggeredSeconds :type Float%20%28double-precision%29) (InputAction :type Input%20Action%20Object%20Reference :default "/Game/Blueprints/FactoryPlayer/Input/InputsMovement/IA_Sprint.IA_Sprint"))
  (:Started
    (bind _sprintdelta (Timeline|Timeline Play)
      (:Update
        _)
      (:Finished
        _))
    (Variables|/Script/Engine.CharacterMovementComponent|SetMaxWalkSpeed (Variables|Character|GetCharacterMovement) (Math|Float|Lerp 5e+02 9e+02 _sprintdelta)))
  (:Completed
    (Timeline|Timeline Reverse)))

(event Input|EnhancedActionEvents|EnhancedInputActionIA_Look
  (params (ActionValue :type Vector%202D%20Structure) (ElapsedSeconds :type Float%20%28double-precision%29) (TriggeredSeconds :type Float%20%28double-precision%29) (InputAction :type Input%20Action%20Object%20Reference :default "/Game/Blueprints/FactoryPlayer/Input/InputsMovement/IA_Look.IA_Look"))
  (Pawn|Input|AddControllerYawInput (.x ActionValue)) ; Left Right Look
  (Pawn|Input|AddControllerPitchInput (.y ActionValue)) ; Up Down Look
)

(event Input|EnhancedActionEvents|EnhancedInputActionIA_Move
  (params (ActionValue :type Vector%202D%20Structure) (ElapsedSeconds :type Float%20%28double-precision%29) (TriggeredSeconds :type Float%20%28double-precision%29) (InputAction :type Input%20Action%20Object%20Reference :default "/Game/Blueprints/FactoryPlayer/Input/InputsMovement/IA_Move.IA_Move"))
  (Pawn|Input|AddMovementInput (Transformation|GetActorRightVector) (.x ActionValue) false)
  (Pawn|Input|AddMovementInput (Transformation|GetActorForwardVector) (.y ActionValue) false))

(event Input|EnhancedActionEvents|EnhancedInputActionIA_Jump
  (params (ActionValue :type Boolean) (ElapsedSeconds :type Float%20%28double-precision%29) (TriggeredSeconds :type Float%20%28double-precision%29) (InputAction :type Input%20Action%20Object%20Reference :default "/Game/Blueprints/FactoryPlayer/Input/InputsMovement/IA_Jump.IA_Jump"))
  (:Started
    (Character|Jump))
  (:Completed
    (Character|StopJumping)))

(event EventBeginPlay
  (bind _asbp_game_instance (Utilities|Casting|CastToBP_GameInstance (Game|GetGameInstance)))
  (Default|LoadInventory (Variables|Default|GetBPC_InventorySystem) (Variables|/Game/Blueprints/SaveData/BP_SaveData_PlayerData.BP_SaveData_PlayerData_C|GetInventoryContent (Variables|/Game/Blueprints/SaveData/BP_GameInstance.BP_GameInstance_C|GetPlayerData _asbp_game_instance))))

(fn ConstructionScript)

(fn RefreshInputs)

(fn GetHud
  (bind _asbp_factory_player_controller (Utilities|Casting|CastToBP_FactoryPlayerController (Pawn|GetController))
    (:then
      (return true (Variables|/Game/Blueprints/FactoryPlayer/BP_FactoryPlayerController.BP_FactoryPlayerController_C|GetHUD _asbp_factory_player_controller)))
    (:CastFailed
      (return false 0))))