(event Custom|AutoSaveAfterAction
  (SaveGame|SaveGametoSlot (Variables|Default|GetLevelData) (Variables|Default|GetLevelDataSlot)))

(event EventBeginPlay
  (CallFunction|InitLevelSaveData)
  (Class|GameplayStatics|SetBaseSoundMix "/Game/Audio/AudioClasses/SCM_AudioMixer.SCM_AudioMixer"))

(event EventEndPlay
  (params (EndPlayReason :type EEndPlayReason%20Enum :default "Destroyed"))
  (SaveGame|SaveGametoSlot (Variables|Default|GetLevelData) (Variables|Default|GetLevelDataSlot)))

(fn ConstructionScript)

(fn LoadLevelData
  (bind _leveldata (Variables|Default|GetLevelData))
  (bind _leveldata_2 (Variables|Default|GetLevelData))
  (bind _containersadded (Variables|/Game/Blueprints/SaveData/BP_SaveData_Level.BP_SaveData_Level_C|GetContainersAdded _leveldata))
  (bind _actorsadded (Variables|/Game/Blueprints/SaveData/BP_SaveData_Level.BP_SaveData_Level_C|GetActorsAdded _leveldata_2))
  (Utilities|FlowControl|Sequence
    (:then_0
      (bind _keys (Utilities|Map|Keys _actorsadded))
      (for _array_element _keys
        (Game|SpawnActorfromClass (Utilities|ResolveSoftReference _array_element) (.Value (Utilities|Map|Find _actorsadded _array_element)) "AlwaysSpawn" "MultiplyWithRoot" 0 0)))
    (:then_1
      (for _array_element_2 (Variables|/Game/Blueprints/SaveData/BP_SaveData_Level.BP_SaveData_Level_C|GetActorsRemoved (Variables|Default|GetLevelData))
        (Utilities|IsValid (Utilities|ResolveSoftReference _array_element_2)
          (:Is%20Valid
            (Actor|DestroyActor (Utilities|ResolveSoftReference _array_element_2))))))
    (:then_2
      (bind _keys_2 (Utilities|Map|Keys _containersadded))
      (for _array_element_3 _keys_2
        (bind _returnvalue (Game|SpawnActorfromClass (Utilities|ResolveSoftReference (.objectclass (.Value (Utilities|Map|Find _containersadded _array_element_3)))) (.transform (.Value (Utilities|Map|Find _containersadded _array_element_3))) "AlwaysSpawn" "MultiplyWithRoot" 0 0))
        (Class|ISaveableObject|LoadObject(Message) _returnvalue (.contents (.Value (Utilities|Map|Find _containersadded _array_element_3))))))))

(fn InitLevelSaveData)

(fn DEBUGPrintAll
  (Utilities|FlowControl|Sequence
    (:then_0
      (Development|PrintString "--- ACTORS ADDED ---")
      (bind _keys (Utilities|Map|Keys (Variables|/Game/Blueprints/SaveData/BP_SaveData_Level.BP_SaveData_Level_C|GetActorsAdded (Variables|Default|GetLevelData))))
      (for _array_element _keys
        (Development|PrintString (Utilities|GetClassDisplayName (Utilities|ResolveSoftReference _array_element)))))
    (:then_1
      (Development|PrintString "--- ACTORS REMOVED ---")
      (for _array_element_2 (Variables|/Game/Blueprints/SaveData/BP_SaveData_Level.BP_SaveData_Level_C|GetActorsRemoved (Variables|Default|GetLevelData))
        (Development|PrintString (Utilities|GetDisplayName (Utilities|ResolveSoftReference _array_element_2)))))
    (:then_2
      (Development|PrintString "--- CONTAINERS ADDED ---")
      (bind _keys_2 (Utilities|Map|Keys (Variables|/Game/Blueprints/SaveData/BP_SaveData_Level.BP_SaveData_Level_C|GetContainersAdded (Variables|Default|GetLevelData))))
      (for _array_element_3 _keys_2
        (Development|PrintString (Utilities|GetDisplayName (Utilities|ResolveSoftReference _array_element_3)))))))