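; Player builder component that handles placing buildings in the factory game, with a build overlay widget shown while enabled.
; Choosing a buildable spawns its actor as a collisionless hologram, yaw-snapped to player facing, with belts using their own offset and trace channel.
; Each tick a camera line trace moves the preview and colors it by validity.
; Building places it and switches controller mode; a separate trace samples existing buildings' data.
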(event Custom|SetEnabled
  (params (Enabled :type Boolean))
  (bind _overlay (Variables|Default|GetOverlay))
  (bind _output_get (Variables|Default|SetEnabled Enabled))
  (if _output_get
    (UserInterface|Viewport|AddtoViewport _overlay 0)
    (else
      (Widget|RemovefromParent _overlay)
      (Variables|Default|SetToBuildData 0)
      (bind _buildpreview (Variables|Default|GetBuildPreview)
        (:then
          (Default|CancelBuild _buildpreview))
        (:else)))))

(event EventBeginPlay
  (bind _returnvalue (UserInterface|CreateWidget "/Game/Blueprints/UI/Overlays/WB_OverlayBuild.WB_OverlayBuild_C"))
  (Variables|Default|SetOverlay _returnvalue))

(event EventTick
  (params (DeltaSeconds :type Float%20%28single-precision%29))
  (if (Variables|Default|GetEnabled)
    (CallFunction|BuildTrace)))

(fn SampleBuilding
  (bind (_success _outhit) (CallFunction|LineTrace "TraceTypeQuery3"))
  (if _success
    (bind _asbp_builds (Utilities|Casting|CastToBP_Builds (.HitActor (Collision|BreakHitResult _outhit)))
      (:then
        (return true (Variables|/Game/Blueprints/Buildings/BP_Builds.BP_Builds_C|GetBuildingData _asbp_builds)))
      (:CastFailed
        _)))
  (return false 0))

(fn BuildTrace
  (bind (_success _outhit) (CallFunction|LineTrace (Variables|Default|GetBuildTraceChannel)))
  (if _success
    (bind _buildpreview (Variables|Default|GetBuildPreview)
      (:then
        (Default|SetAllMaterials _buildpreview (select (Default|IsBuildable _buildpreview) "/Game/Assets/Holograms/M_HologramPlace.M_HologramPlace" "/Game/Assets/Holograms/M_HologramPlaceInvalid.M_HologramPlaceInvalid") false)
        (Default|UpdateLocation _buildpreview _outhit))
      (:else))
    (else
      (bind _buildpreview_2 (Variables|Default|GetBuildPreview)
        (:then
          (Default|UpdateLocationInvalid _buildpreview_2))
        (:else)))))

(fn LineTrace
  (params (TraceChannel :type ETraceTypeQuery%20Enum :default "TraceTypeQuery1"))
  (bind _returnvalue (Game|GetPlayerCameraManager 0))
  (bind _returnvalue_2 (Transformation|GetActorLocation _returnvalue))
  (bind (_outhit _returnvalue_3) (Collision|LineTraceByChannel _returnvalue_2 (+ _returnvalue_2 (* (Transformation|GetActorForwardVector _returnvalue) (Variables|Default|GetBuildRange))) TraceChannel false (Utilities|Array|MakeArray (Components|GetOwner) (Variables|Default|GetBuildPreview)) "None"))
  (if _returnvalue_3
    (return true _outhit)
    (else
      (return false ""))))

(fn Build
  (params (KeyDown :type Boolean))
  (if KeyDown
    (bind _buildpreview (Variables|Default|GetBuildPreview)
      (:then
        (if (Default|IsBuildable _buildpreview)
          (bind _success (Default|PlaceBuild (Variables|Default|GetBuildPreview)))
          (if _success
            (Variables|Default|SetBuildPreview 0)
            (Audio|PlaySound2D "/Engine/EditorSounds/GamePreview/EjectFromPlayer_Cue.EjectFromPlayer_Cue" 1.0 1.0 0.0 0 0)
            (if false ; Place Another?
              (CallFunction|SpawnBuild)
              (else
                (bind _asbp_factory_player_controller (Utilities|Casting|CastToBP_FactoryPlayerController (Game|GetPlayerController 0)))
                (Default|SetMode _asbp_factory_player_controller "NewEnumerator0"))))))
      (:else))))

(fn SettoBuild
  (params (BuildableID :type DA%20Buildable%20Object%20Reference))
  (bind _output_get (Variables|Default|SetToBuildData BuildableID))
  (Default|SettoBuild (Variables|Default|GetOverlay) _output_get (Variables|Default|GetPlayerInventory))
  (CallFunction|SpawnBuild))

(fn AddRotation
  (params (CustomRot :type Boolean) (MouseInput :type Float%20%28double-precision%29))
  (bind _buildpreview (Variables|Default|GetBuildPreview))
  (if CustomRot
    (Default|ScrollBuildCustom _buildpreview MouseInput)
    (else
      (Default|ScrollBuild _buildpreview MouseInput))))

(fn SpawnBuild
  (bind _buildpreview (Variables|Default|GetBuildPreview)
    (:then
      (Default|CancelBuild _buildpreview))
    (:else
      _))
  (Variables|Default|GetToBuildData
    (:then
      (bind _returnvalue (Game|SpawnActorfromClass (Variables|/Game/Blueprints/Buildings/DA_Buildable.DA_Buildable_C|GetBuildClass (Variables|Default|GetToBuildData)) (Math|Transform|MakeTransform "0.000000,0.000000,-10000.000000" (Math|Rotator|MakeRotator 0.0 0.0 (Math|Float|SnapToGrid(Float) (+ (.yaw (Transformation|GetActorRotation (Game|Player|GetPlayerPawn 0))) (Math|Float|SelectFloat 1.8e+02 -9e+01 (== (Variables|Default|GetToBuildData) "/Game/FactoryData/BuildableData/Belting/DA_Build_Belt.DA_Build_Belt"))) 45.0)) "1.000000,1.000000,1.000000") "Undefined" "MultiplyWithRoot" 0 0 0))
      (Variables|Default|SetBuildPreview _returnvalue)
      (Default|SetAllMaterials (Variables|Default|GetBuildPreview) "/Game/Assets/Holograms/M_HologramPlace.M_HologramPlace" false)
      (Default|UpdateCollision (Variables|Default|GetBuildPreview) "NoCollision")
      (Variables|Default|SetBuildTraceChannel (select (== (Variables|Default|GetToBuildData) "/Game/FactoryData/BuildableData/Belting/DA_Build_Belt.DA_Build_Belt") "TraceTypeQuery1" "TraceTypeQuery6")))
    (:else)))