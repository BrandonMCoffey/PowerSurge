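; BP_DroppedItemStack is an item stack lying in the world that players can pick up, with a hover prompt showing the item name and, for stacks, its quantity.
; Interacting adds the stack to the player's inventory component and destroys the actor on success.
; SaveItem records its transform, class and contents in the game mode's ContainersAdded level data, Destroyed removes that entry, and both trigger an autosave.
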(event Custom|InteractWith_1_1
  (params (PlayerCharacter :type BP%20Factory%20FPS%20Character%20Object%20Reference))
  (bind _bpc_inventorysystem (Variables|/Game/Blueprints/Player/BP_FactoryFPSCharacter.BP_FactoryFPSCharacter_C|GetBPC_InventorySystem PlayerCharacter))
  (Utilities|IsValid _bpc_inventorysystem
    (:Is%20Valid
      (bind _success (Default|AddtoInventory _bpc_inventorysystem (Variables|Default|GetItemID) (Variables|Default|GetQuantity)))
      (if _success
        (Actor|DestroyActor)))))

(event Custom|SaveItem
  (bind _asbp_factory_game_mode (Utilities|Casting|CastToBP_FactoryGameMode (Game|GetGameMode)))
  (Utilities|Map|Add (Variables|/Game/Blueprints/SaveData/BP_SaveData_Level.BP_SaveData_Level_C|GetContainersAdded (Variables|/Game/Blueprints/Player/BP_FactoryGameMode.BP_FactoryGameMode_C|GetLevelData _asbp_factory_game_mode)) (Utilities|ResolveSoftReference self) (Utilities|Struct|MakeFSaveableObjectStruct (Transformation|GetActorTransform) "/Game/Blueprints/Inventory/BP_DroppedItemStack.BP_DroppedItemStack_C" (Utilities|Array|MakeArray (Utilities|Struct|MakeFInventorySlotStruct (Variables|Default|GetItemID) (Variables|Default|GetQuantity)))))
  (Default|AutoSaveAfterAction _asbp_factory_game_mode))

(event EventDestroyed
  (bind _asbp_factory_game_mode (Utilities|Casting|CastToBP_FactoryGameMode (Game|GetGameMode)))
  (Utilities|Map|Remove (Variables|/Game/Blueprints/SaveData/BP_SaveData_Level.BP_SaveData_Level_C|GetContainersAdded (Variables|/Game/Blueprints/Player/BP_FactoryGameMode.BP_FactoryGameMode_C|GetLevelData _asbp_factory_game_mode)) (Utilities|ResolveSoftReference self))
  (Default|AutoSaveAfterAction _asbp_factory_game_mode))

(fn ConstructionScript)

(fn InteractHover
  (bind _itemid (Variables|Default|GetItemID))
  (bind _name (Variables|/Game/Blueprints/Items/DA_Items.DA_Items_C|GetName _itemid))
  (return (select (> (Variables|Default|GetQuantity) 1) (Utilities|Text|FormatText "Pick Up {quantity} {item}" (Variables|Default|GetQuantity) _name) (Utilities|Text|FormatText "Pick up {item}" _name))))

(fn Interactwith
  (params (PlayerCharacter :type BP%20Factory%20FPS%20Character%20Object%20Reference))
  (return false))